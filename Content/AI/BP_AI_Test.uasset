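; BP_AI_Test is a test AI actor that fights with an axe and exposes its combat stats.
; On BeginPlay it spawns a BP_Axe, snaps it to the mesh's hand socket, disables its pickup collision and registers it with BPCCombat as the equipped weapon.
; Getter functions return the weapon's base, thrust and slash damage, the mesh, and the actor's thrust and slash resistances.
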(event `self.ReceiveBeginPlay`
  (`parent.ReceiveBeginPlay`)
  (bind _returnvalue (`|SpawnActorFromClass` "/Game/Blueprints/Weapons/BP_Axe.BP_Axe_C" (`KismetMathLibrary.MakeTransform` (0.0 0.0 0.0)) "Undefined" "OverrideRootScale" self true self))
  (bind _output_get (set `self.Weapon` _returnvalue))
  (`self.K2_AttachToComponent` _output_get (`self.Mesh`) "handSocketAxe" "SnapToTarget" "SnapToTarget" "SnapToTarget" true)
  (`PrimitiveComponent.SetCollisionEnabled` (`/Game/Blueprints/Weapons/BP_Weapon.WeaponItemPickup` _output_get) "NoCollision")
  (`/Game/Blueprints/BPC_Combat.SetEquippedWeapon` (`self.BPC_Combat`) _output_get))

(fn `GetDmgFromWeapon`
  (returns (BaseDmg :type "Float (double-precision)") (Thrust :type "Float (double-precision)") (Slash :type "Float (double-precision)"))
  (bind (_basedmg _thrust _slash) (`/Game/Blueprints/Weapons/BP_Weapon.GetDamage` (`self.Weapon`)))
  (return _basedmg _thrust _slash))

(fn `GetMesh`
  (returns (SkeletalMesh :type "SkeletalMeshComponent Object Reference"))
  (return (`self.Mesh`)))

(fn `GetResistance`
  (returns (ResistanceThrust :type "Float (double-precision)") (ResistanceSlash :type "Float (double-precision)"))
  (return (`self.ResistanceThrust`) (`self.ResistanceSlash`)))

(fn `UserConstructionScript`
  (`parent.UserConstructionScript`))