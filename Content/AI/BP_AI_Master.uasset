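; Base AI enemy character that chases perceived attackable targets and can be stunned, lock-on targeted or killed by one-hit KOs.
; Perception writes PlayerTarget to the Blackboard, using roam-area and distance limits plus a memory timer before clearing it and flagging GoBack.
; BeginPlay initializes abilities and binds attributes to a health widget shown with the lock-on indicator.
; One-hit KOs trigger an impulse-driven ragdoll, while stuns play a montage with movement disabled.
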(event `self.ReceiveBeginPlay`
  (`BlackboardComponent.SetValueAsVector` (`AIBlueprintHelperLibrary.GetBlackboard` null) "StartLocation" (`self.K2_GetActorLocation`))
  (`/Game/Blueprints/Abilities/BPC_Ability.InitAbilities` (`self.BPC_Ability`) (`self.Known Abilities`))
  (bind _asui_enemy_health (cast `/Game/Widgets/UI_EnemyHealth` (`WidgetComponent.GetUserWidgetObject` (`self.HealthBar`))))
  (bind _output_get (set `self.HealthWidget` _asui_enemy_health))
  (set `/Game/Widgets/UI_EnemyHealth.Attributes` (`self.BPC_Attributes`) _output_get)
  (`Widget.SetVisibility` _output_get "Hidden")
  (`self.LockOnIndicatorShow` false))

(event `RecieveHit`
  (params (`One-Hit-KO` :type Boolean) (HitBoneName :type Name) (ImpactVector :type "Vector Structure"))
  (bind _mesh (`self.Mesh`))
  (bind _mesh_2 (`self.Mesh`))
  (if `One-Hit-KO`
    (`/Engine/EditorBlueprintResources/StandardMacros.DoOnce` false
      (:`Completed`
        (`PrimitiveComponent.SetCollisionProfileName` _mesh_2 "Ragdoll" true)
        (`PrimitiveComponent.SetSimulatePhysics` _mesh_2 true)
        (`PrimitiveComponent.SetCollisionEnabled` (`self.CapsuleComponent`) "NoCollision")
        (if (`SceneComponent.IsSimulatingPhysics` _mesh HitBoneName)
          (`PrimitiveComponent.AddImpulseAtLocation` _mesh ImpactVector (`self.K2_GetActorLocation`) HitBoneName)
          (`/Game/Blueprints/GameplayTags/BPC_GameplayTags.AddTag` :`self` (`self.BPC_GameplayTags`) :`TagToAdd` (struct :`TagName` "State.Dead")))))))

(event `DoStunThing`
  (`|PlayMontage` (`self.Mesh`) "/Game/Animations/Player/Combat/Death_Montage.Death_Montage"
    (:`then`
      (`MovementComponent.StopMovementImmediately` (`self.CharacterMovement`))
      (`CharacterMovementComponent.DisableMovement` (`self.CharacterMovement`)))
    (:`OnCompleted`
      (`CharacterMovementComponent.SetMovementMode` (`self.CharacterMovement`) "MOVE_Walking" 0 :!label _label))
    (:`OnInterrupted`
      (goto _label))))

(event `self.AIPerception.OnPerceptionUpdated`
  (params (UpdatedActors :type "Array of Actor Object Reference (by ref)"))
  (bind _returnvalue (`AIBlueprintHelperLibrary.GetBlackboard` null))
  (for _array_element UpdatedActors
    (bind _canbeattacked (message `/Game/Blueprints/BPI_CharacterUtilityFunc.CanBeAttacked` _array_element))
    (if _canbeattacked
      (bind _info (`AIPerceptionComponent.GetActorsPerception` (`self.AIPerception`) _array_element))
      (bind (_target _lastsensedstimuli) (break `ActorPerceptionBlueprintInfo` _info))
      (for _array_element_2 _lastsensedstimuli
        (if (`.bSuccessfullySensed` (break `AIStimulus` _array_element_2))
          (`/Engine/EditorBlueprintResources/StandardMacros.IsValid` _returnvalue
            (:`Is Valid`
              (bind _returnvalue_2 (and (>= (`KismetMathLibrary.Vector_Distance` (`self.K2_GetActorLocation` _target) (`BlackboardComponent.GetValueAsVector` _returnvalue "RoamLocation")) (`self.AreaDistanceToStopFollowing`)) (>= (`self.GetDistanceTo` _target) (`self.PlayerDistanceToStopFollowing`))))
              (if (not _returnvalue_2)
                (`BlackboardComponent.SetValueAsObject` (`AIBlueprintHelperLibrary.GetBlackboard` null) "PlayerTarget" _target)
                (`KismetSystemLibrary.K2_ClearAndInvalidateTimerHandle` (`self.RememberPlayerTimerRef`))))
            (:`Is Not Valid`
              (`self.StopFollowingPlayer` :!label _label_2)
              (`KismetSystemLibrary.K2_ClearAndInvalidateTimerHandle` (`self.RememberPlayerTimerRef`))))
          (else
            (`/Engine/EditorBlueprintResources/StandardMacros.IsValid` _returnvalue
              (:`Is Valid`
                (if _returnvalue_2
                  (bind _returnvalue_3 (`KismetSystemLibrary.K2_SetTimerDelegate` (delegate `StopFollowingPlayer`) (`self.MemoryDuration`)))
                  (set `self.RememberPlayerTimerRef` _returnvalue_3)))
              (:`Is Not Valid`
                (goto _label_2)))))))))

(event `StopFollowingPlayer`
  (bind _returnvalue (`AIBlueprintHelperLibrary.GetBlackboard` null))
  (`/Engine/EditorBlueprintResources/StandardMacros.IsValid` _returnvalue
    (:`Is Valid`
      (`BlackboardComponent.SetValueAsObject` _returnvalue "PlayerTarget" null)
      (`BlackboardComponent.SetValueAsBool` (`AIBlueprintHelperLibrary.GetBlackboard` null) "GoBack" true)
      (`KismetSystemLibrary.K2_ClearAndInvalidateTimerHandle` (`self.RememberPlayerTimerRef`)))
    (:`Is Not Valid`
      (`KismetSystemLibrary.K2_ClearAndInvalidateTimerHandle` (`self.RememberPlayerTimerRef`)))))

(event `self.LockOnIndicatorShow`
  (params (Show :type Boolean))
  (bind _healthwidget (`self.HealthWidget`))
  (`SceneComponent.SetHiddenInGame` (`self.LockOnIndicator`) (not Show) false)
  (if Show
    (`Widget.SetVisibility` _healthwidget "Visible")
    (else
      (`Widget.SetVisibility` _healthwidget "Hidden"))))

(event `self.DisableAIMovement`
  (`CharacterMovementComponent.DisableMovement` (`self.CharacterMovement`)))

(fn `CanBeAttacked`
  (returns (CanBeAttacked :type Boolean))
  (return false))

(fn `CanBeLockedOn`
  (returns (CanLock :type Boolean))
  (return true))

(fn `GetDmgFromWeapon`
  (returns (BaseDmg :type "Float (double-precision)") (Thrust :type "Float (double-precision)") (Slash :type "Float (double-precision)"))
  (return 0.0 0.0 0.0))

(fn `GetInventoryMeneger`
  (returns (InveneotryRef :type "/Game/Blueprints/Inventory/BPC_InventoryMenager Object Reference"))
  (return null))

(fn `GetMesh`
  (returns (SkeletalMesh :type "SkeletalMeshComponent Object Reference"))
  (return (`self.Mesh`)))

(fn `GetPlayer`
  (returns (Player :type "/Game/Blueprints/BP_ThirdPersonCharacter Object Reference"))
  (return null))

(fn `GetResistance`
  (returns (ResistanceThrust :type "Float (double-precision)") (ResistanceSlash :type "Float (double-precision)"))
  (return (`self.ResistanceThrust`) (`self.ResistanceSlash`)))

(fn `GetWeaponType`
  (returns (WeaponType :type "/Game/Blueprints/Weapons/Enum_Weapons Enum"))
  (return "NewEnumerator0"))

(fn `Stun`
  (returns (Success :type Boolean))
  (`self.StopAnimMontage` null)
  (`self.DoStunThing`)
  (`KismetSystemLibrary.PrintString` "STUN")
  (return true))

(fn `UserConstructionScript`)