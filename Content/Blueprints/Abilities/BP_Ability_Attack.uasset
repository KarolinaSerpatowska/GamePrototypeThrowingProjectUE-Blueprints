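; Melee attack ability that plays light or heavy combo sections of a shared montage on the owner's mesh, for spear or axe.
; Attacks start only while a combo window is open or the montage is idle, and disable aiming until the ability ends.
; External calls set the attack type, advance or reset the next section names, and open or close the window.
; Owner communication runs through message calls, including restoring movement speed once the montage stops.
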(event `self.ReceiveBeginPlay`
  (`parent.ReceiveBeginPlay`)
  (set `self.LightComboAttack` (`self.DefaultLightComboAttack`))
  (set `self.HeavyComboAttack` (`self.DefaultHeavyComboAttack`)))

(event `self.UseAbility`
  (bind _returnvalue (`self.GetOwner`))
  (bind _skeletalmesh (message `/Game/Blueprints/BPI_CharacterUtilityFunc.GetMesh` (`self.GetOwner`)))
  (if (or (`self.AttackWindowOpen`) (not (`AnimInstance.Montage_IsPlaying` (`SkeletalMeshComponent.GetAnimInstance` _skeletalmesh) "/Game/Animations/Player/Combat/Axe/Combo_Montage.Combo_Montage")))
    (message `/Game/Blueprints/BPI_CharacterUtilityFunc.SetCanAim` _returnvalue false)
    (bind _weapontype (message `/Game/Blueprints/BPI_CharacterUtilityFunc.GetWeaponType` _returnvalue))
    (switch `/Game/Blueprints/Enum_AttackTypes` (`self.AttackType`)
      (:`NewEnumerator0`
        (switch `/Game/Blueprints/Weapons/Enum_Weapons` _weapontype
          (:`NewEnumerator1`
            (set `self.AnimMontage` "/Game/Animations/Player/Combat/Axe/Combo_Montage.Combo_Montage"))
          (:`NewEnumerator2`
            (set `self.AnimMontage` "/Game/Animations/Player/Combat/Axe/Combo_Montage.Combo_Montage")))
        (bind _skeletalmesh_2 (message `/Game/Blueprints/BPI_CharacterUtilityFunc.GetMesh` (`self.GetOwner`)))
        (`/Engine/EditorBlueprintResources/StandardMacros.IsValid` _skeletalmesh_2
          (:`Is Valid`
            (bind _animmontage (`self.AnimMontage`)
              (:`then`
                (`|PlayMontage` _skeletalmesh_2 _animmontage 1.0 0.0 (`self.LightComboAttack`)
                  (:`OnCompleted`
                    _)
                  (:`OnInterrupted`
                    _)))
              (:`else`
                _)))
          (:`Is Not Valid`
            _))
        (`self.EndAbility`))
      (:`NewEnumerator1`
        (switch `/Game/Blueprints/Weapons/Enum_Weapons` _weapontype
          (:`NewEnumerator1`
            (set `self.AnimMontage` "/Game/Animations/Player/Combat/Axe/Combo_Montage.Combo_Montage"))
          (:`NewEnumerator2`
            (set `self.AnimMontage` "/Game/Animations/Player/Combat/Axe/Combo_Montage.Combo_Montage")))
        (bind _skeletalmesh_3 (message `/Game/Blueprints/BPI_CharacterUtilityFunc.GetMesh` (`self.GetOwner`)))
        (`/Engine/EditorBlueprintResources/StandardMacros.IsValid` _skeletalmesh_3
          (:`Is Valid`
            (bind _animmontage_2 (`self.AnimMontage`)
              (:`then`
                (`|PlayMontage` _skeletalmesh_3 _animmontage_2 1.0 0.0 (`self.HeavyComboAttack`)
                  (:`OnCompleted`
                    _)
                  (:`OnInterrupted`
                    _)))
              (:`else`
                _)))
          (:`Is Not Valid`
            _))
        (`self.EndAbility`)))))

(event `self.EndAbility`
  (bind _returnvalue (`self.GetOwner`))
  (`parent.EndAbility`)
  (message `/Game/Blueprints/BPI_CharacterUtilityFunc.SetCanAim` _returnvalue true)
  (bind _skeletalmesh (message `/Game/Blueprints/BPI_CharacterUtilityFunc.GetMesh` (`self.GetOwner`)))
  (if (not (`AnimInstance.Montage_IsPlaying` (`SkeletalMeshComponent.GetAnimInstance` _skeletalmesh) "/Game/Animations/Player/Combat/Axe/Combo_Montage.Combo_Montage"))
    (message `/Game/Blueprints/BPI_CharacterUtilityFunc.ResetMovementSpeed` _returnvalue)))

(event `/Game/Blueprints/BPI_AttackUtility.SetAttackType`
  (params (AttackType :type "/Game/Blueprints/Enum_AttackTypes Enum" :default "NewEnumerator0"))
  (set `self.AttackType` AttackType))

(event `/Game/Blueprints/BPI_AttackUtility.SetDefaultCombo`
  (set `self.LightComboAttack` (`self.DefaultLightComboAttack`))
  (set `self.HeavyComboAttack` (`self.DefaultHeavyComboAttack`))
  (set `self.AttackWindowOpen` false))

(event `/Game/Blueprints/BPI_AttackUtility.SetNextComboSegment`
  (params (LightCombo :type Name) (HeavyCombo :type Name))
  (set `self.LightComboAttack` LightCombo)
  (set `self.HeavyComboAttack` HeavyCombo)
  (set `self.AttackWindowOpen` true)
  (message `/Game/Blueprints/BPI_CharacterUtilityFunc.SetCanUseLeftMouse` (`self.GetOwner`)))

(fn `UserConstructionScript`
  (`parent.UserConstructionScript`))