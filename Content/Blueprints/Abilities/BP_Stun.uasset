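; Stun ability that turns the owner's weapon at inventory index 1 into a stun hitbox, usable only while that weapon is equipped.
; On use, it snaps its Sphere to that weapon's LodgePoint and enables query-only overlaps.
; Overlapped actors receive StunMessage, and a true result or the ability ending returns the sphere to the ability root with collision disabled.
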(event `self.UseAbility`
  (bind _sphere (`self.Sphere`))
  (bind _lodgepoint (`/Game/Blueprints/Weapons/BP_Weapon.LodgePoint` (`|GetArrayItem` (`/Game/Blueprints/Inventory/BPC_InventoryMenager.WeaponsOnCharacter` (`self.GetComponentByClass` (`self.GetOwner`) "/Game/Blueprints/Inventory/BPC_InventoryMenager.BPC_InventoryMenager_C")) 1)))
  (`parent.UseAbility`)
  (`SceneComponent.K2_SetWorldLocation` _sphere (`SceneComponent.K2_GetComponentLocation` _lodgepoint) false false)
  (`SceneComponent.K2_AttachToComponent` (`self.Sphere`) _lodgepoint "None" "SnapToTarget" "SnapToTarget" "SnapToTarget" true)
  (`PrimitiveComponent.SetCollisionEnabled` _sphere "QueryOnly")
  (`KismetSystemLibrary.PrintString` "YESSSSSSSSSSS"))

(event `self.Sphere.OnComponentBeginOverlap`
  (params (OverlappedComponent :type "PrimitiveComponent Object Reference") (OtherActor :type "Actor Object Reference") (OtherComp :type "PrimitiveComponent Object Reference") (OtherBodyIndex :type Integer) (bFromSweep :type Boolean) (SweepResult :type "HitResult Structure (by ref)"))
  (bind _success (message `/Game/Blueprints/BPI_EnemyUtility.Stun` OtherActor))
  (if _success
    (`SceneComponent.K2_DetachFromComponent` (`self.Sphere`) "KeepWorld" "KeepWorld" "KeepWorld" true)
    (`SceneComponent.K2_AttachToComponent` (`self.Sphere`) (`self.DefaultSceneRoot`) "None" "SnapToTarget" "SnapToTarget" "SnapToTarget" true)
    (`PrimitiveComponent.SetCollisionEnabled` (`self.Sphere`) "NoCollision")))

(event `self.EndAbility`
  (`parent.EndAbility`)
  (`SceneComponent.K2_DetachFromComponent` (`self.Sphere`) "KeepWorld" "KeepWorld" "KeepWorld" true)
  (`SceneComponent.K2_AttachToComponent` (`self.Sphere`) (`self.DefaultSceneRoot`) "None" "SnapToTarget" "SnapToTarget" "SnapToTarget" true)
  (`PrimitiveComponent.SetCollisionEnabled` (`self.Sphere`) "NoCollision"))

(fn `FinalUseAllowanceCheck`
  (returns (CanUse :type Boolean))
  (bind _returnvalue (`self.GetComponentByClass` (`self.GetOwner`) "/Game/Blueprints/Inventory/BPC_InventoryMenager.BPC_InventoryMenager_C"))
  (if (== (`/Game/Blueprints/Inventory/BPC_InventoryMenager.EquipedWeapon` _returnvalue) (`|GetArrayItem` (`/Game/Blueprints/Inventory/BPC_InventoryMenager.WeaponsOnCharacter` _returnvalue) 1))
    (return true)
    (else
      (return false))))

(fn `UserConstructionScript`
  (`parent.UserConstructionScript`))