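; Spear ability that creates a 30-second buff zone at the location of the owner's first weapon.
; On use it moves a sphere to the weapon and enables overlap queries, sending EnableBuffMessage to actors entering or leaving.
; A timer then disables the sphere and clears the owner's buff.
; Use requires a valid inventory component, a teleportable-to weapon and the owner within DistanceForUsing of it.
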(event `self.UseAbility`
  (`parent.UseAbility`)
  (`SceneComponent.K2_SetWorldLocation` (`self.Sphere`) (`self.K2_GetActorLocation` (`|GetArrayItem` (`/Game/Blueprints/Inventory/BPC_InventoryMenager.WeaponsOnCharacter` (`self.GetComponentByClass` (`self.GetOwner`) "/Game/Blueprints/Inventory/BPC_InventoryMenager.BPC_InventoryMenager_C")))) false false)
  (`PrimitiveComponent.SetCollisionEnabled` (`self.Sphere`) "QueryOnly")
  (`KismetSystemLibrary.K2_SetTimerDelegate` (delegate `BuffDone`) 30.0))

(event `BuffDone`
  (message `/Game/Blueprints/BPI_CharacterUtilityFunc.EnableBuff` (`self.GetOwner`) 0.0)
  (`PrimitiveComponent.SetCollisionEnabled` (`self.Sphere`) "NoCollision"))

(event `self.Sphere.OnComponentBeginOverlap`
  (params (OverlappedComponent :type "PrimitiveComponent Object Reference") (OtherActor :type "Actor Object Reference") (OtherComp :type "PrimitiveComponent Object Reference") (OtherBodyIndex :type Integer) (bFromSweep :type Boolean) (SweepResult :type "HitResult Structure (by ref)"))
  (message `/Game/Blueprints/BPI_CharacterUtilityFunc.EnableBuff` OtherActor 0.9)
  (`KismetSystemLibrary.PrintString` "KEKEKEKEKEKEKEKEKEKEKEKEEKEKE"))

(event `self.Sphere.OnComponentEndOverlap`
  (params (OverlappedComponent :type "PrimitiveComponent Object Reference") (OtherActor :type "Actor Object Reference") (OtherComp :type "PrimitiveComponent Object Reference") (OtherBodyIndex :type Integer))
  (message `/Game/Blueprints/BPI_CharacterUtilityFunc.EnableBuff` OtherActor 0.0)
  (`KismetSystemLibrary.PrintString` "KEKEKEKEKEKEKEKEKEKEKEKEEKEKE"))

(fn `FinalUseAllowanceCheck`
  (returns (CanUse :type Boolean))
  (bind _returnvalue (`self.GetOwner`))
  (bind _returnvalue_2 (`self.GetComponentByClass` _returnvalue "/Game/Blueprints/Inventory/BPC_InventoryMenager.BPC_InventoryMenager_C"))
  (bind _output (`|GetArrayItem` (`/Game/Blueprints/Inventory/BPC_InventoryMenager.WeaponsOnCharacter` _returnvalue_2)))
  (`/Engine/EditorBlueprintResources/StandardMacros.IsValid` _returnvalue_2
    (:`Is Valid`
      (bind _canteleport (message `/Game/Blueprints/Weapons/BPI_ThrowableWeapon.CanTeleportTo` _output))
      (if (and _canteleport (<= (`self.GetDistanceTo` _returnvalue _output) (`self.DistanceForUsing`)))
        (return true)
        (else
          _)))
    (:`Is Not Valid`
      _))
  (return false))

(fn `UserConstructionScript`
  (`parent.UserConstructionScript`))