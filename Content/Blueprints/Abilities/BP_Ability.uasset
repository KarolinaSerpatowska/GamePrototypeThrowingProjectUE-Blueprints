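; Base ability Blueprint that gates use on its owner's gameplay tags and plays an animation montage.
; An attempt passes FinalUseAllowanceCheck (true by default), then checks prevention and required tags on BPC_GameplayTags, passing both if that component is absent.
; Use adds UseAddingTags to the owner and plays the montage on the owner-provided mesh.
; EndAbility removes those tags on completion or interruption, or immediately without a valid mesh or montage.
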(event `AttempUseAbility`
  (bind _canuseability (`self.CanUseAbility`))
  (if _canuseability
    (`self.UseAbilityPreStep`)))

(event `UseAbilityPreStep`
  (for _array_element (`self.UseAddingTags`)
    (`self.AddAbilityTag` _array_element))
  (`self.UseAbility`))

(event `UseAbility`
  (bind _skeletalmesh (message `/Game/Blueprints/BPI_CharacterUtilityFunc.GetMesh` (`self.GetOwner`)))
  (`/Engine/EditorBlueprintResources/StandardMacros.IsValid` _skeletalmesh
    (:`Is Valid`
      (bind _animmontage (`self.AnimMontage`)
        (:`then`
          (`|PlayMontage` _skeletalmesh _animmontage
            (:`OnCompleted`
              _)
            (:`OnInterrupted`
              _)))
        (:`else`
          _)))
    (:`Is Not Valid`
      _))
  (`self.EndAbility`))

(event `EndAbility`
  (for _array_element (`self.UseAddingTags`)
    (`self.RemoveAbilityTag` _array_element)))

(fn `AddAbilityTag`
  (params (AbilityTag :type "GameplayTag Structure"))
  (bind _returnvalue (`self.GetOwner`))
  (bind _returnvalue_2 (`self.GetComponentByClass` _returnvalue "/Game/Blueprints/GameplayTags/BPC_GameplayTags.BPC_GameplayTags_C"))
  (`/Engine/EditorBlueprintResources/StandardMacros.IsValid` _returnvalue_2
    (:`Is Valid`
      (`/Game/Blueprints/GameplayTags/BPC_GameplayTags.AddTag` _returnvalue_2 AbilityTag (make `/Game/Blueprints/S_WhoDoneThis` _returnvalue (`self.GetInstigatorController`)))
      (return))))

(fn `CanUseAbility`
  (returns (CanUseAbility :type Boolean))
  (bind _canuse (`self.FinalUseAllowanceCheck`))
  (if _canuse
    (bind _isrestricted (`self.IsUsingAbilityRestricted`))
    (if _isrestricted
      (return false)
      (else
        (bind _isallowed (`self.IsUsingAbilityPrerequisitesFullfiled`))
        (if _isallowed
          (return true)
          (else
            (return false)))))
    (else
      (return false))))

(fn `FinalUseAllowanceCheck`
  (returns (CanUse :type Boolean))
  (return true))

(fn `IsUsingAbilityPrerequisitesFullfiled`
  (returns (IsAllowed :type Boolean))
  (bind _returnvalue (`self.GetComponentByClass` (`self.GetOwner`) "/Game/Blueprints/GameplayTags/BPC_GameplayTags.BPC_GameplayTags_C"))
  (`/Engine/EditorBlueprintResources/StandardMacros.IsValid` _returnvalue
    (:`Is Valid`
      (bind _tagcontainer (`/Game/Blueprints/GameplayTags/BPC_GameplayTags.GetActiveTagContainer` _returnvalue))
      (return (`BlueprintGameplayTagLibrary.HasAllTags` _tagcontainer (`self.UseRequiredTags`))))
    (:`Is Not Valid`
      (return true))))

(fn `IsUsingAbilityRestricted`
  (returns (IsRestricted :type Boolean))
  (bind _returnvalue (`self.GetComponentByClass` (`self.GetOwner`) "/Game/Blueprints/GameplayTags/BPC_GameplayTags.BPC_GameplayTags_C"))
  (`/Engine/EditorBlueprintResources/StandardMacros.IsValid` _returnvalue
    (:`Is Valid`
      (bind _tagcontainer (`/Game/Blueprints/GameplayTags/BPC_GameplayTags.GetActiveTagContainer` _returnvalue))
      (return (`BlueprintGameplayTagLibrary.HasAnyTags` _tagcontainer (`self.UsePreventionTags`))))
    (:`Is Not Valid`
      (return false))))

(fn `RemoveAbilityTag`
  (params (AbilityTag :type "GameplayTag Structure"))
  (bind _returnvalue (`self.GetOwner`))
  (bind _returnvalue_2 (`self.GetComponentByClass` _returnvalue "/Game/Blueprints/GameplayTags/BPC_GameplayTags.BPC_GameplayTags_C"))
  (`/Engine/EditorBlueprintResources/StandardMacros.IsValid` _returnvalue_2
    (:`Is Valid`
      (`/Game/Blueprints/GameplayTags/BPC_GameplayTags.RemoveTag` _returnvalue_2 AbilityTag (make `/Game/Blueprints/S_WhoDoneThis` _returnvalue (`self.GetInstigatorController`)))
      (return))))

(fn `UserConstructionScript`)