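; BPC_Ability is a component that manages the set of abilities available to its owning Pawn.
; Each ability is an actor spawned from a class with the Pawn as Owner and Instigator, and each addition broadcasts the changed list.
; InitAbilities destroys existing ability actors and rebuilds the list from known classes.
; UseAbility passes an attack type to the ability at an index, then attempts to use it.
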(event `self.ReceiveBeginPlay`
  (bind _aspawn (cast `Pawn` (`self.GetOwner`)))
  (set `self.OnwerRefPawn` _aspawn))

(fn `AddAbilityByClass`
  (params (AbilityClass :type "/Game/Blueprints/Abilities/BP_Ability Class Reference"))
  (locals (NewLocalVar_0 :type "Array of /Game/Blueprints/Abilities/BP_Ability Object Reference"))
  (bind _onwerrefpawn (`self.OnwerRefPawn`))
  (bind _returnvalue (`|SpawnActorFromClass` AbilityClass (`KismetMathLibrary.MakeTransform` (0.0 0.0 0.0)) "Undefined" "OverrideRootScale" _onwerrefpawn _onwerrefpawn))
  (`KismetArrayLibrary.Array_Add` (`self.AvailableAbilities`) _returnvalue)
  (`self.AbilitiesAvailableChanged` (`self.AvailableAbilities`))
  (return))

(fn `InitAbilities`
  (params (KnownAbilities :type "Array of /Game/Blueprints/Abilities/BP_Ability Class Reference"))
  (bind _availableabilities (`self.AvailableAbilities`))
  (for _array_element _availableabilities
    (`/Engine/EditorBlueprintResources/StandardMacros.IsValid` _array_element
      (:`Is Valid`
        (`Actor.K2_DestroyActor` _array_element))))
  (`KismetArrayLibrary.Array_Clear` _availableabilities)
  (for _array_element_2 KnownAbilities
    (`self.AddAbilityByClass` _array_element_2))
  (return))

(fn `UseAbility`
  (params (AbilityIndex :type Integer) (AttackType :type "/Game/Blueprints/Enum_AttackTypes Enum" :default "NewEnumerator0"))
  (bind _output (`|GetArrayItem` (`self.AvailableAbilities`) AbilityIndex))
  (message `/Game/Blueprints/BPI_AttackUtility.SetAttackType` _output AttackType)
  (`/Game/Blueprints/Abilities/BP_Ability.AttempUseAbility` _output)
  (return))