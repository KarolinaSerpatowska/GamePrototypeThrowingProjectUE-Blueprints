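; BP_Sacriface is a sacrifice ability that passes a health amount and a temporary buff to its owning actor.
; UseAbility calls the parent, sends SacrifaceMessage to the owner, then after a fixed delay prints a debug string and sends the buff removal message.
; FinalUseAllowanceCheck permits use only when the owner's BPC_InventoryMenager has the first weapon in WeaponsOnCharacter equipped.
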(event `self.UseAbility`
  (bind _returnvalue (`self.GetOwner`))
  (`parent.UseAbility`)
  (message `/Game/Blueprints/BPI_CharacterUtilityFunc.Sacriface` _returnvalue 100.0 0.5)
  (`KismetSystemLibrary.Delay` 5.0)
  (`KismetSystemLibrary.PrintString` "Done")
  (message `/Game/Blueprints/BPI_CharacterUtilityFunc.RemoveBuffSacriface` _returnvalue))

(fn `FinalUseAllowanceCheck`
  (returns (CanUse :type Boolean))
  (bind _returnvalue (`self.GetComponentByClass` (`self.GetOwner`) "/Game/Blueprints/Inventory/BPC_InventoryMenager.BPC_InventoryMenager_C"))
  (`/Engine/EditorBlueprintResources/StandardMacros.IsValid` _returnvalue
    (:`Is Valid`
      (if (== (`|GetArrayItem` (`/Game/Blueprints/Inventory/BPC_InventoryMenager.WeaponsOnCharacter` _returnvalue)) (`/Game/Blueprints/Inventory/BPC_InventoryMenager.EquipedWeapon` _returnvalue))
        (return true)
        (else
          _)))
    (:`Is Not Valid`
      _))
  (return false))

(fn `UserConstructionScript`
  (`parent.UserConstructionScript`))