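; AI attack ability that plays a horizontal melee montage on the owner's mesh.
; UseAbility gets the mesh through the owner's GetMeshMessage call and ends the ability when the montage completes or is interrupted, or at once if the mesh is invalid.
; FinalUseAllowanceCheck blocks use while the owner's death montage is playing.
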(event `self.UseAbility`
  (bind _skeletalmesh (message `/Game/Blueprints/BPI_CharacterUtilityFunc.GetMesh` (`self.GetOwner`)))
  (`/Engine/EditorBlueprintResources/StandardMacros.IsValid` _skeletalmesh
    (:`Is Valid`
      (`|PlayMontage` _skeletalmesh "/Game/Animations/Player/Combat/Axe/MeleeAttackHorizontal_Montage.MeleeAttackHorizontal_Montage"
        (:`OnCompleted`
          _)
        (:`OnInterrupted`
          _)))
    (:`Is Not Valid`
      _))
  (`self.EndAbility`))

(fn `FinalUseAllowanceCheck`
  (returns (CanUse :type Boolean))
  (bind _skeletalmesh (message `/Game/Blueprints/BPI_CharacterUtilityFunc.GetMesh` (`self.GetOwner`)))
  (if (not (`AnimInstance.Montage_IsPlaying` (`SkeletalMeshComponent.GetAnimInstance` _skeletalmesh) "/Game/Animations/Player/Combat/Death_Montage.Death_Montage"))
    (return true)
    (else
      (return false))))

(fn `UserConstructionScript`
  (`parent.UserConstructionScript`))