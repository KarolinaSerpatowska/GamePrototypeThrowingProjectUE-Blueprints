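; Teleport ability that moves its owner to the location of a weapon from the owner's inventory manager component.
; On use it runs the parent ability logic, then sets the owner's location to the first entry in WeaponsOnCharacter, without sweep.
; It overrides the final use check to require a valid inventory component, the weapon's approval via CanTeleportToMessage, and a distance within DistanceForUsing.
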(event `self.UseAbility`
  (bind _returnvalue (`self.GetOwner`))
  (`parent.UseAbility`)
  (`self.K2_SetActorLocation` _returnvalue (`self.K2_GetActorLocation` (`|GetArrayItem` (`/Game/Blueprints/Inventory/BPC_InventoryMenager.WeaponsOnCharacter` (`self.GetComponentByClass` _returnvalue "/Game/Blueprints/Inventory/BPC_InventoryMenager.BPC_InventoryMenager_C")))) false false))

(fn `FinalUseAllowanceCheck`
  (returns (CanUse :type Boolean))
  (bind _returnvalue (`self.GetOwner`))
  (bind _returnvalue_2 (`self.GetComponentByClass` _returnvalue "/Game/Blueprints/Inventory/BPC_InventoryMenager.BPC_InventoryMenager_C"))
  (bind _output (`|GetArrayItem` (`/Game/Blueprints/Inventory/BPC_InventoryMenager.WeaponsOnCharacter` _returnvalue_2)))
  (`/Engine/EditorBlueprintResources/StandardMacros.IsValid` _returnvalue_2
    (:`Is Valid`
      (bind _canteleport (message `/Game/Blueprints/Weapons/BPI_ThrowableWeapon.CanTeleportTo` _output))
      (if (and _canteleport (<= (`self.GetDistanceTo` _returnvalue _output) (`self.DistanceForUsing`)))
        (return true)
        (else
          _)))
    (:`Is Not Valid`
      _))
  (return false))

(fn `UserConstructionScript`
  (`parent.UserConstructionScript`))