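; Blueprint function library with shared helpers for weapon socket lookup and attribute math.
; Two switch functions convert between socket point types and names for axe, spear and sword, though the name-to-point lookup has no sword case.
; CalculateAttributeValue combines an attribute's base, delta and multiplier through a math expression, then clamps the result between zero and the attribute's maximum.
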(fn GetSocketNamebyPoint
  (params (Type :type Enum_AttachPoint%20Enum :default "NewEnumerator0"))
  (switch Utilities|FlowControl|Switch|SwitchonEnum_AttachPoint Type
    (:NewEnumerator0
      (return "AxeSocket"))
    (:NewEnumerator1
      (return "SpearSocket"))
    (:NewEnumerator2
      (return "SwordSocket"))))

(fn GetPointNamebySocket
  (params (Name :type Name))
  (switch name Name
    (:AxeSocket
      (return "NewEnumerator0"))
    (:SpearSocket
      (return "NewEnumerator1"))))

(fn CalculateAttributeValue
  (params (Attribute :type S%20Attributes%20Structure))
  (bind (_basevalue _delta _multiplier _max) (Utilities|Struct|BreakS_Attributes Attribute))
  (return (Math|Float|Clamp(Float) (|((Base+Delta)*Multiplier) _basevalue _delta _multiplier) 0.0 _max)))