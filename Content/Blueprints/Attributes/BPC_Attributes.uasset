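; BPC_Attributes is an attribute component that stores a Health attribute with base, delta, multiplier and max values.
; A DetermineAttribute macro routes gameplay tags to the matching attribute for lookup, change and listener binding, currently handling only Health.
; ChangeAttribute adds the value to the chosen field, then broadcasts a health-changed dispatcher with a context struct holding the attribute, change and instigator.
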(event `Signature` :!signature `self.AttributeHealthChanged`
  (params (AttributeContext :type "/Game/Blueprints/Attributes/S_AttributesContext Structure")))

(fn `AddAtributeListener`
  (params (AttributeTag :type "GameplayTag Structure") (Event :type "Delegate (by ref)"))
  (`self.DetermineAttribute` AttributeTag
    (:`Health`
      (add `self.AttributeHealthChanged` Event))))

(fn `ChangeAttribute`
  (params (AttributeTag :type "GameplayTag Structure") (ValueChange :type "Float (double-precision)") (AttributeTypeToChange :type "/Game/Blueprints/Attributes/Enum_Attribute Enum" :default "NewEnumerator0") (WhoDoneThis :type "/Game/Blueprints/S_WhoDoneThis Structure"))
  (`self.DetermineAttribute` AttributeTag
    (:`Health`
      (`self.ChangeAttributeValue` (`self.Health`) ValueChange AttributeTypeToChange)
      (bind _context (`self.CreateAttributeContext` (`self.Health`) (`local.ValueChange`) (`local.WhoDoneThis`)))
      (`self.AttributeHealthChanged` _context)
      (return))))

(fn `ChangeAttributeValue`
  (params (AttributeToChange :type "/Game/Blueprints/Attributes/S_Attributes Structure (by ref)") (ValueChange :type "Float (double-precision)") (AttributeTypeToChange :type "/Game/Blueprints/Attributes/Enum_Attribute Enum" :default "NewEnumerator0"))
  (bind (_basevalue _delta _multiplier _max) (break `/Game/Blueprints/Attributes/S_Attributes` AttributeToChange))
  (switch `/Game/Blueprints/Attributes/Enum_Attribute` AttributeTypeToChange
    (:`NewEnumerator0`
      (return))
    (:`NewEnumerator1`
      (setmembers `/Game/Blueprints/Attributes/S_Attributes` :`StructRef` AttributeToChange :`BaseValue` (+ _basevalue (`local.ValueChange`))))
    (:`NewEnumerator2`
      (setmembers `/Game/Blueprints/Attributes/S_Attributes` :`StructRef` AttributeToChange :`Delta` (+ _delta (`local.ValueChange`))))
    (:`NewEnumerator3`
      (setmembers `/Game/Blueprints/Attributes/S_Attributes` :`StructRef` AttributeToChange :`Multiplier` (+ _multiplier (`local.ValueChange`))))
    (:`NewEnumerator4`
      (setmembers `/Game/Blueprints/Attributes/S_Attributes` :`StructRef` AttributeToChange :`Max` (+ _max (`local.ValueChange`)))))
  (return))

(fn `CreateAttributeContext`
  (params (AttributeChanged :type "/Game/Blueprints/Attributes/S_Attributes Structure") (ValueChange :type "Float (double-precision)") (WhoDoneThis :type "/Game/Blueprints/S_WhoDoneThis Structure"))
  (returns (Context :type "/Game/Blueprints/Attributes/S_AttributesContext Structure"))
  (return (make `/Game/Blueprints/Attributes/S_AttributesContext` AttributeChanged ValueChange WhoDoneThis)))

(fn `GetAttributeFromTag`
  (params (TagSearchedFor :type "GameplayTag Structure"))
  (returns (AttributeFound :type "/Game/Blueprints/Attributes/S_Attributes Structure"))
  (locals (LocalAttributeFound :type "/Game/Blueprints/Attributes/S_Attributes Structure"))
  (`self.DetermineAttribute` TagSearchedFor
    (:`Health`
      (bind _output_get (set `local.LocalAttributeFound` (`self.Health`)))
      (return _output_get))))