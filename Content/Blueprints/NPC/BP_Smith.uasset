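; Blacksmith NPC that lets the player open the smith screen of their inventory UI when nearby.
; Sphere overlap identifies the player through GetPlayerMessage, caches the reference, enables input on the actor, shows the interact widget and opens a Gate.
; Pressing E passes through that Gate to call OpenSmith on the player's UIInventory.
; Leaving the sphere disables input, hides the widget and closes the Gate.
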(event `Key|E`
  (params (Key :type "Key Structure"))
  (:`Pressed`
    (`/Engine/EditorBlueprintResources/StandardMacros.Gate` true :!label _label
      (:`Exit`
        (`/Game/Widgets/UI_Inventory.OpenSmith` (`/Game/Blueprints/BP_ThirdPersonCharacter.UIInventory` (`self.Player`)))))))

(event `self.Sphere.OnComponentBeginOverlap`
  (params (OverlappedComponent :type "PrimitiveComponent Object Reference") (OtherActor :type "Actor Object Reference") (OtherComp :type "PrimitiveComponent Object Reference") (OtherBodyIndex :type Integer) (bFromSweep :type Boolean) (SweepResult :type "HitResult Structure (by ref)"))
  (bind _player (message `/Game/Blueprints/BPI_CharacterUtilityFunc.GetPlayer` OtherActor))
  (`/Engine/EditorBlueprintResources/StandardMacros.IsValid` _player
    (:`Is Valid`
      (set `self.Player` _player)
      (`self.EnableInput` (`GameplayStatics.GetPlayerController` 0))
      (`SceneComponent.SetHiddenInGame` (`self.InteractWidget`) false false)
      (goto _label :!via `Open`))))

(event `self.Sphere.OnComponentEndOverlap`
  (params (OverlappedComponent :type "PrimitiveComponent Object Reference") (OtherActor :type "Actor Object Reference") (OtherComp :type "PrimitiveComponent Object Reference") (OtherBodyIndex :type Integer))
  (bind _player (message `/Game/Blueprints/BPI_CharacterUtilityFunc.GetPlayer` OtherActor))
  (`/Engine/EditorBlueprintResources/StandardMacros.IsValid` _player
    (:`Is Valid`
      (`self.DisableInput` (`GameplayStatics.GetPlayerController` 0))
      (`SceneComponent.SetHiddenInGame` (`self.InteractWidget`) true false)
      (goto _label :!via `Close`))))

(fn `UserConstructionScript`)