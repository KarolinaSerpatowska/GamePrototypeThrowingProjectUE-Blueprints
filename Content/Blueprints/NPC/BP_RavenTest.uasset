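; BP_RavenTest is a test raven NPC that follows a player reference supplied through Init.
; While following is enabled, FollowPlayer re-runs every 0.2 seconds, issuing an AI move toward the player when far and calling Land, or targeting itself when close.
; SetFollowPlayer only sets the flag; it does not start the loop.
; Despawn moves the capsule high along Z over several seconds, prints a debug message and destroys the actor.
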(event `self.FollowPlayer`
  (if (`self.FollowPlayer?`)
    (if (>= (`self.GetDistanceTo` (`self.Player`)) 400.0)
      (`|AIMoveTo` self (0.0 0.0 0.0) (`self.Player`) 10.0
        (:`then`
          (`self.Land`)))
      (else
        (`|AIMoveTo` self (0.0 0.0 0.0) self
          (:`then`
            _))))
    (`KismetSystemLibrary.Delay` 0.2)
    (`self.FollowPlayer`)))

(event `self.Despawn`
  (`KismetSystemLibrary.MoveComponentTo` (`self.CapsuleComponent`) (0.0 0.0 5000.0) (struct) false false 5.0)
  (`KismetSystemLibrary.PrintString` "YES IM DONE")
  (`self.K2_DestroyActor`))

(event `self.Init`
  (params (Player :type "/Game/Blueprints/BP_ThirdPersonCharacter Object Reference"))
  (set `self.Player` Player))

(event `self.SetFollowPlayer`
  (params (FollowPlayer :type Boolean))
  (set `self.FollowPlayer?` FollowPlayer))

(fn `UserConstructionScript`)