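; BP_CheckPoint is an interactable checkpoint that refills the player's healing charges to the maximum when E is pressed nearby.
; A sphere overlap identifies the player through GetPlayerMessage, caches the reference, shows the interact widget and enables input on the actor.
; A Gate opened and closed by the overlap events guards the key press, which then updates the HUD and inventory healing displays.
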(event `Key|E`
  (params (Key :type "Key Structure"))
  (bind _player (`self.Player`))
  (bind _maxhealings (`/Game/Blueprints/BP_ThirdPersonCharacter.MaxHealings` _player))
  (:`Pressed`
    (`/Engine/EditorBlueprintResources/StandardMacros.Gate` true :!label _label
      (:`Exit`
        (bind _output_get (set `/Game/Blueprints/BP_ThirdPersonCharacter.AvailableHealings` _maxhealings _player))
        (`/Game/Widgets/UI_HUD.HealingUpdate` (`/Game/Blueprints/BP_ThirdPersonCharacter.HUD` _player) _output_get)
        (`/Game/Widgets/UI_Inventory.UpdateHealingText` (`/Game/Blueprints/BP_ThirdPersonCharacter.UIInventory` _player) _output_get _maxhealings)))))

(event `self.Sphere.OnComponentBeginOverlap`
  (params (OverlappedComponent :type "PrimitiveComponent Object Reference") (OtherActor :type "Actor Object Reference") (OtherComp :type "PrimitiveComponent Object Reference") (OtherBodyIndex :type Integer) (bFromSweep :type Boolean) (SweepResult :type "HitResult Structure (by ref)"))
  (bind _player (message `/Game/Blueprints/BPI_CharacterUtilityFunc.GetPlayer` OtherActor))
  (`/Engine/EditorBlueprintResources/StandardMacros.IsValid` _player
    (:`Is Valid`
      (set `self.Player` _player)
      (`self.EnableInput` (`GameplayStatics.GetPlayerController` 0))
      (`SceneComponent.SetHiddenInGame` (`self.InteractWidget`) false false)
      (goto _label :!via `Open`))))

(event `self.Sphere.OnComponentEndOverlap`
  (params (OverlappedComponent :type "PrimitiveComponent Object Reference") (OtherActor :type "Actor Object Reference") (OtherComp :type "PrimitiveComponent Object Reference") (OtherBodyIndex :type Integer))
  (bind _player (message `/Game/Blueprints/BPI_CharacterUtilityFunc.GetPlayer` OtherActor))
  (`/Engine/EditorBlueprintResources/StandardMacros.IsValid` _player
    (:`Is Valid`
      (`self.DisableInput` (`GameplayStatics.GetPlayerController` 0))
      (`SceneComponent.SetHiddenInGame` (`self.InteractWidget`) true false)
      (goto _label :!via `Close`))))

(fn `UserConstructionScript`)