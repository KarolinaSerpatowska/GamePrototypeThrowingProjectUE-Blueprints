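; Throwable weapon that the player charges, throws and picks back up with E once landed.
; Fire adds a projectile movement component at charge-scaled speed, while a timeline drives gravity and line traces along velocity.
; Hits lodge the weapon at a normal-adjusted point and attach it to the actor, one-hit killing AI at the struck bone.
; Flying too far or staying lodged too long spawns a raven that carries it toward the player.
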(event `RavenLand`
  (`KismetSystemLibrary.PrintString` "HIIIII")
  (`PrimitiveComponent.SetCollisionEnabled` (`self.PickupCollision`) "QueryAndPhysics")
  (set `self.WeaponState` "NewEnumerator2"))

(event `StartTracing`
  (bind _returnvalue (`self.K2_GetActorLocation`))
  (bind _weaponmesh (`self.WeaponMesh`))
  (bind _ai_ref (`self.AI_ref`))
  (bind _player (`self.Player`))
  (bind _raven (`self.Raven`))
  (bind (_returnvalue_x _returnvalue_y) (`KismetMathLibrary.BreakVector` (`self.K2_GetActorLocation` _player)))
  ;[1 1 1] trace hit and land
  (`TimelineComponent.SetPlayRate` (`self.Tracing`) 4.0)
  (bind (_direction _newtrack_0) (`Timeline|Tracing` :!via `PlayFromStart` :!label _label)
    (:`Update`
      (if (> (`self.GetDistanceTo` (`self.Player`)) 10000.0)
        (bind _projectilemovement (`self.ProjectileMovement`)
          (:`then`
            (`ActorComponent.K2_DestroyComponent` _projectilemovement)
            (`self.StopTracing`)
            (`PrimitiveComponent.SetCollisionEnabled` (`self.PickupCollision`) "QueryAndPhysics")
            (`SceneComponent.K2_SetRelativeRotation` :`self` (`self.Root`))
            (`/Game/Blueprints/Weapons/BPI_Weapon.StopRotation`)
            (`self.K2_DetachFromActor` "KeepWorld" "KeepWorld" "KeepWorld")
            (bind _returnvalue_2 (`AIBlueprintHelperLibrary.SpawnAIFromClass` "/Game/Blueprints/NPC/BP_RavenTest.BP_RavenTest_C" null (`KismetMathLibrary.MakeVector` _returnvalue_x _returnvalue_y 5000.0) (struct) false null))
            (bind _asbp_raven_test (cast `/Game/Blueprints/NPC/BP_RavenTest` _returnvalue_2))
            (set `self.Raven` _asbp_raven_test)
            (set `/Game/Blueprints/NPC/BP_RavenTest.Player` _player (`self.Raven`))
            (`self.K2_AttachToComponent` (`Character.Mesh` (`self.Raven`)) "None" "SnapToTarget" "SnapToTarget" "SnapToTarget")
            (set `/Game/Blueprints/NPC/BP_RavenTest.FollowPlayer?` true _raven)
            (add `/Game/Blueprints/NPC/BP_RavenTest.Land` _raven (delegate `RavenLand`))
            (message `/Game/Blueprints/NPC/BPI_RavenUtility.FollowPlayer` (`self.Raven`)))
          (:`else`))
        (else
          (bind _projectilemovement_2 (`self.ProjectileMovement`)
            (:`then`
              (set `ProjectileMovementComponent.ProjectileGravityScale` _newtrack_0 _projectilemovement_2)
              (bind _outhit (`KismetSystemLibrary.LineTraceSingle` :`Start` _returnvalue :`End` (+ _returnvalue (* (`KismetMathLibrary.Normal` (`self.GetVelocity`)) (`self.ThrowTraceDistance`))) :`TraceChannel` "TraceTypeQuery1" :`DrawDebugType` "ForDuration" :`DrawTime` 12.0))
              (bind (_bblockinghit _binitialoverlap _time _distance _location _impactpoint _normal _impactnormal _physmat _hitactor _hitcomponent _hitbonename) (`GameplayStatics.BreakHitResult` _outhit))
              (if _bblockinghit
                (set `self.ImpactPoint` _impactpoint)
                (set `self.ImpactNormal` _impactnormal)
                (set `self.Hit Actor` _hitactor)
                (set `self.Hit Bone Name` _hitbonename)
                (`self.StopTracing`)
                (`self.LandWeapon`)
                (`PrimitiveComponent.SetCollisionResponseToChannel` _weaponmesh "ECC_WorldStatic" "ECR_Block")
                (`PrimitiveComponent.SetCollisionResponseToChannel` _weaponmesh "ECC_Pawn" "ECR_Block")
                ;[1 1 1] ai to change
                (bind _asbp_ai_master (cast `/Game/AI/BP_AI_Master` (`self.Hit Actor`))
                  (:`then`
                    (set `self.AI_ref` _asbp_ai_master)
                    (`self.K2_AttachToComponent` (`Character.Mesh` (`self.AI_ref`)) (`self.Hit Bone Name`) "SnapToTarget" "SnapToTarget" "SnapToTarget")
                    (`/Game/AI/BP_AI_Master.RecieveHit` _ai_ref true (`self.Hit Bone Name`) (* (`KismetMathLibrary.Normal` (- (`self.K2_GetActorLocation` _ai_ref) (`self.CameraLocation`))) 20000.0)))
                  (:`CastFailed`
                    (`self.K2_AttachToActor` (`self.Hit Actor`) "None" "KeepWorld" "KeepWorld" "KeepWorld")))))
            (:`else`)))))))

(event `self.ReceiveBeginPlay`
  (`parent.ReceiveBeginPlay`)
  (set `self.WeaponState` "NewEnumerator0")
  (bind _asui_interaction_indicator (cast `/Game/Widgets/UI_InteractionIndicator` (`WidgetComponent.GetUserWidgetObject` (`self.PickupIndicator`))))
  (bind _output_get (set `self.UIInteraction Indicator` _asui_interaction_indicator))
  (`Widget.SetVisibility` _output_get "Hidden"))

(event `StopTracing`
  ;[1 1 1] trace hit and land
  (goto _label :!via `Stop`))

(event `/Game/Blueprints/Weapons/BPI_ThrowableWeapon.StartCharge`
  ;[1 1 1] charging
  (set `self.WeaponState` "NewEnumerator3")
  (if (or (`|EnumEquality` (`self.WeaponState`) "NewEnumerator0") (`|EnumEquality` (`self.WeaponState`) "NewEnumerator3"))
    (`TimelineComponent.SetPlayRate` (`self.ChargeTimeline`) 1.0)
    (bind (_direction _chargeamount) (`Timeline|ChargeTimeline` :!label _label_2)
      (:`Update`
        (set `self.ThrowChargeAmount` _chargeamount)))))

(event `StopCharge`
  ;[1 1 1] charging
  (if (or (`|EnumEquality` (`self.WeaponState`) "NewEnumerator0") (`|EnumEquality` (`self.WeaponState`) "NewEnumerator3"))
    (`|ExecutionSequence`
      (:`then_0`
        (goto _label_2 :!via `Stop`))
      (:`then_1`
        (goto _label_2 :!via `SetNewTime`)))))

(event `LandWeapon`
  (bind _projectilemovement (`self.ProjectileMovement`)
    (:`then`
      (`ActorComponent.K2_DestroyComponent` _projectilemovement)
      (`self.Lodge`))
    (:`else`
      _))
  (`PrimitiveComponent.SetCollisionEnabled` (`self.PickupCollision`) "QueryAndPhysics")
  (bind _returnvalue (`KismetSystemLibrary.K2_SetTimerDelegate` (delegate `BringWeapon`) 180.0))
  (set `self.TimerHandle` _returnvalue))

(event `/Game/Blueprints/Weapons/BPI_ThrowableWeapon.EndCharge`
  ;[1 1 1] charging
  (if (or (`|EnumEquality` (`self.WeaponState`) "NewEnumerator0") (`|EnumEquality` (`self.WeaponState`) "NewEnumerator3"))
    (set `self.WeaponState` "NewEnumerator0")
    (goto _label_2 :!via `Reverse`)))

(event `BringWeapon`
  (bind (_returnvalue_x _returnvalue_y _returnvalue_z) (`KismetMathLibrary.BreakVector` (`self.K2_GetActorLocation`)))
  (`KismetSystemLibrary.PrintString` "KEKEKEKEKEEKEKEKEKE")
  (`PrimitiveComponent.SetCollisionResponseToChannel` (`self.WeaponMesh`) "ECC_Pawn" "ECR_Ignore")
  (`self.K2_DetachFromActor` "KeepWorld" "KeepWorld" "KeepWorld")
  (bind _returnvalue (`AIBlueprintHelperLibrary.SpawnAIFromClass` "/Game/Blueprints/NPC/BP_RavenTest.BP_RavenTest_C" null (`KismetMathLibrary.MakeVector` _returnvalue_x _returnvalue_y _returnvalue_z) (struct) false null))
  (bind _asbp_raven_test (cast `/Game/Blueprints/NPC/BP_RavenTest` _returnvalue))
  (set `self.Raven` _asbp_raven_test)
  (set `/Game/Blueprints/NPC/BP_RavenTest.Player` (`self.Player`) (`self.Raven`))
  (`self.K2_AttachToComponent` (`Character.Mesh` (`self.Raven`)) "None" "SnapToTarget" "SnapToTarget" "SnapToTarget")
  (set `/Game/Blueprints/NPC/BP_RavenTest.FollowPlayer?` true (`self.Raven`))
  (message `/Game/Blueprints/NPC/BPI_RavenUtility.FollowPlayer` (`self.Raven`)))

(event `/Game/Blueprints/Weapons/BPI_ThrowableWeapon.Fire`
  (params (AimDirection :type "Vector Structure") (InitialRotation :type "Rotator Structure") (CameraLocation :type "Vector Structure"))
  (set `self.CameraLocation` CameraLocation)
  (`self.K2_DetachFromActor` "KeepWorld" "KeepWorld" "KeepWorld")
  (set `self.ThrowDirection` (`KismetMathLibrary.InverseTransformDirection` (`self.GetTransform`) AimDirection))
  (set `self.WeaponState` "NewEnumerator1")
  (bind _returnvalue (`AddComponent|NODE_AddProjectileMovementComponent-2`))
  (bind _output_get (set `self.ProjectileMovement` _returnvalue))
  (set `ProjectileMovementComponent.ProjectileGravityScale` 0.0 _output_get)
  (set `ProjectileMovementComponent.bRotationFollowsVelocity` true _output_get)
  (`ProjectileMovementComponent.SetVelocityInLocalSpace` _output_get (* (`self.ThrowDirection`) (`KismetMathLibrary.Lerp` (`self.MinCharge`) (`self.MaxCharge`) (`self.ThrowChargeAmount`))))
  (set `self.ThrowChargeAmount` 0.0)
  (`self.StopCharge`)
  (`self.StartTracing`))

(event `Key|E`
  (params (Key :type "Key Structure"))
  (bind _weaponmesh (`self.WeaponMesh`))
  ;[1 1 1] pickup weapon
  (:`Pressed`
    (`/Engine/EditorBlueprintResources/StandardMacros.Gate` true :!label _label_3
      (:`Exit`
        (`/Game/Blueprints/BP_ThirdPersonCharacter.PickupAnimation` (`self.Player`))
        (`PrimitiveComponent.SetCollisionResponseToChannel` (`self.WeaponMesh`) "ECC_Pawn" "ECR_Ignore")
        (`self.K2_DetachFromActor` "KeepRelative")
        (`KismetSystemLibrary.K2_ClearAndInvalidateTimerHandle` (`self.TimerHandle`))
        (`/Game/Blueprints/Weapons/BPI_ThrowableWeapon.AttachWeaponAfterThrow`)
        (`PrimitiveComponent.SetCollisionResponseToChannel` _weaponmesh "ECC_WorldStatic" "ECR_Overlap")
        (`PrimitiveComponent.SetCollisionResponseToChannel` _weaponmesh "ECC_Pawn" "ECR_Ignore")
        (`PrimitiveComponent.SetCollisionEnabled` (`self.PickupCollision`) "NoCollision")
        (`Widget.SetVisibility` (`self.UIInteraction Indicator`) "Hidden")
        (set `self.WeaponState` "NewEnumerator0")
        (`SceneComponent.K2_SetRelativeRotation` :`self` (`self.LodgePoint`))
        (`SceneComponent.K2_SetRelativeRotation` :`self` (`self.Pivot`))
        (bind _raven (`self.Raven`)
          (:`then`
            (set `/Game/Blueprints/NPC/BP_RavenTest.FollowPlayer?` false _raven)
            (message `/Game/Blueprints/NPC/BPI_RavenUtility.Despawn` _raven)
            (set `self.Raven` null))
          (:`else`))))))

(event `self.PickupCollision.OnComponentBeginOverlap`
  (params (OverlappedComponent :type "PrimitiveComponent Object Reference") (OtherActor :type "Actor Object Reference") (OtherComp :type "PrimitiveComponent Object Reference") (OtherBodyIndex :type Integer) (bFromSweep :type Boolean) (SweepResult :type "HitResult Structure (by ref)"))
  ;[1 1 1] pickup weapon
  (if (`|EnumEquality` (`self.WeaponState`) "NewEnumerator2")
    (if (== OtherActor (`self.Player`))
      (`self.EnableInput` (`GameplayStatics.GetPlayerController` 0))
      (`Widget.SetVisibility` (`self.UIInteraction Indicator`) "Visible")
      (goto _label_3 :!via `Open`))))

(event `self.PickupCollision.OnComponentEndOverlap`
  (params (OverlappedComponent :type "PrimitiveComponent Object Reference") (OtherActor :type "Actor Object Reference") (OtherComp :type "PrimitiveComponent Object Reference") (OtherBodyIndex :type Integer))
  (if (`|EnumEquality` (`self.WeaponState`) "NewEnumerator2")
    (if (== OtherActor (`self.Player`))
      (`self.DisableInput` (`GameplayStatics.GetPlayerController` 0))
      (`Widget.SetVisibility` (`self.UIInteraction Indicator`) "Hidden")
      (goto _label_3 :!via `Close`))))

(event `/Game/Blueprints/Weapons/BPI_ThrowableWeapon.AttachWeaponAfterThrow`
  (bind _socketname (`/Game/Blueprints/MyFunctionLibrary.GetSocketNameByPoint` (`self.AttachPoint`)))
  (bind _skeletalmesh (`/Game/Blueprints/BPI_CharacterUtilityFunc.GetMesh` (`self.Player`)))
  (`self.K2_AttachToComponent` _skeletalmesh _socketname "KeepWorld" "KeepWorld" "KeepWorld")
  (`self.K2_SetActorTransform` (`SceneComponent.GetSocketTransform` _skeletalmesh _socketname "RTS_World")))

(fn `AdjustImpactLocation`
  (params (ImpactNormal :type "Vector Structure") (ImpactLocation :type "Vector Structure"))
  (returns (ReturnValue :type "Vector Structure"))
  (bind (_returnvalue_roll _returnvalue_pitch) (`KismetMathLibrary.BreakRotator` (`KismetMathLibrary.MakeRotationFromAxes` ImpactNormal)))
  (bind _returnvalue (* (/ (- 90.0 (`KismetMathLibrary.SelectFloat` _returnvalue_pitch 0.0 (> _returnvalue_pitch 0.0))) 90.0) 10.0))
  (set `self.ZAdjustment` _returnvalue)
  (return (+ (+ ImpactLocation (`KismetMathLibrary.MakeVector` 0.0 0.0 _returnvalue)) (- (`self.K2_GetActorLocation`) (`SceneComponent.K2_GetComponentLocation` (`self.LodgePoint`))))))

(fn `CanBeEquiped`
  (returns (CanEquip :type Boolean))
  (if (`|EnumEquality` (`self.WeaponState`) "NewEnumerator0")
    (return true)
    (else
      (return false))))

(fn `CanTeleportTo`
  (returns (CanTeleport :type Boolean))
  (return false))

(fn `CanThrow`
  (returns (CanThrow :type Boolean))
  (bind _weaponstate (`self.WeaponState`))
  (if (or (`|EnumEquality` _weaponstate "NewEnumerator0") (`|EnumEquality` _weaponstate "NewEnumerator3"))
    (return true)
    (else
      (return false))))

(fn `Lodge`
  (`KismetSystemLibrary.PrintString` "lodge")
  (`SceneComponent.K2_SetRelativeRotation` (`self.LodgePoint`) (`KismetMathLibrary.MakeRotator` (`KismetMathLibrary.RandomFloatInRange` -3.0 -8.0)) false false)
  (`self.K2_SetActorLocation` (`self.AdjustImpactLocation` (`self.ImpactNormal`) (`self.ImpactPoint`)))
  (set `self.WeaponState` "NewEnumerator2")
  (set `self.WeaponMainState` "NewEnumerator0"))

(fn `UserConstructionScript`
  (`parent.UserConstructionScript`)
  (`PrimitiveComponent.SetCollisionEnabled` (`self.PickupCollision`) "NoCollision"))