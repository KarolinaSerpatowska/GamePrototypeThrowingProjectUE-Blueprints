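; Modular spear weapon built from base, head, cubes and lower-head skeletal meshes, with the attached parts following the weapon mesh through master pose.
; ChangeWeaponParts swaps each mesh from WeaponInfo selections, using Gungnir or axe meshes.
; The cubes and lower-head choices also write the player's ability slots (spear buff or none, teleport or sacrifice) and reinitialise the ability component.
; CanTeleportTo allows teleporting only in one specific weapon state.
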(event `self.ReceiveBeginPlay`
  (`parent.ReceiveBeginPlay`)
  (`PrimitiveComponent.SetCollisionEnabled` (`self.WeaponItemPickup`) "NoCollision"))

(fn `CanTeleportTo`
  (returns (CanTeleport :type Boolean))
  (return (`|EnumEquality` (`self.WeaponState`) "NewEnumerator2")))

(fn `ChangeWeaponParts`
  (bind (_weaponinfo_weapontype _weaponinfo_canbethrown _weaponinfo_weaponname _weaponinfo_baseselection _weaponinfo_bladeselection _weaponinfo_isequipped _weaponinfo_somethingselection _weaponinfo_bladedownselection) (break `/Game/Blueprints/Weapons/S_WeaponInfo` (`self.WeaponInfo`)))
  (bind _knownabilities (`/Game/Blueprints/BP_ThirdPersonCharacter.KnownAbilities` (`self.Player`)))
  (bind _knownabilities_2 (`/Game/Blueprints/BP_ThirdPersonCharacter.KnownAbilities` (`self.Player`)))
  (`parent.ChangeWeaponParts`)
  (`|ExecutionSequence`
    (:`then_0`
      (switch `/Game/Blueprints/Weapons/Enum_BaseSelection` _weaponinfo_baseselection
        (:`NewEnumerator0`
          (`SkinnedMeshComponent.SetSkinnedAssetAndUpdate` (`self.WeaponMesh`) "/Game/Meshes/Weapon/Modular/Gungnir/Base/Gungnir_base.Gungnir_base" false))
        (:`NewEnumerator2`
          (`SkinnedMeshComponent.SetSkinnedAssetAndUpdate` (`self.WeaponMesh`) "/Game/Meshes/Weapon/Modular/Axe/Basic/axe_basicBLADE.axe_basicBLADE" false))))
    (:`then_1`
      (switch `/Game/Blueprints/Weapons/Enum_BladeSelection` _weaponinfo_bladeselection
        (:`NewEnumerator0`
          (`SkinnedMeshComponent.SetSkinnedAssetAndUpdate` (`self.HeadMesh`) "/Game/Meshes/Weapon/Modular/Gungnir/Base/Gungnir_headUP.Gungnir_headUP" false))
        (:`NewEnumerator1`
          (`SkinnedMeshComponent.SetSkinnedAssetAndUpdate` (`self.HeadMesh`) "/Game/Meshes/Weapon/Modular/Axe/Basic/axe_basic.axe_basic" false))))
    (:`then_2`
      (switch `/Game/Blueprints/Weapons/Enum_SomethingSelection` _weaponinfo_somethingselection
        (:`NewEnumerator0`
          (`SkinnedMeshComponent.SetSkinnedAssetAndUpdate` (`self.CubesHeadMesh`) "/Game/Meshes/Weapon/Modular/Gungnir/Base/Gungnir_Cubes.Gungnir_Cubes" false)
          (set `self.AbilityToAdd` "/Game/Blueprints/Abilities/BP_SpearBuff.BP_SpearBuff_C"))
        (:`NewEnumerator2`
          (`SkinnedMeshComponent.SetSkinnedAssetAndUpdate` (`self.CubesHeadMesh`) "/Game/Meshes/Weapon/Modular/Axe/Basic/axe_basic.axe_basic" false)
          (set `self.AbilityToAdd` null)))
      (if (`KismetArrayLibrary.Array_IsValidIndex` _knownabilities 2)
        (`KismetArrayLibrary.Array_Set` _knownabilities 2 (`self.AbilityToAdd`))
        (else
          (`KismetArrayLibrary.Array_Add` _knownabilities (`self.AbilityToAdd`))))
      (`/Game/Blueprints/Abilities/BPC_Ability.InitAbilities` (`/Game/Blueprints/BP_ThirdPersonCharacter.BPC_Ability` (`self.Player`)) _knownabilities))
    (:`then_3`
      (switch `/Game/Blueprints/Weapons/Enum_BladeDownSelection` _weaponinfo_bladedownselection
        (:`NewEnumerator0`
          (`SkinnedMeshComponent.SetSkinnedAssetAndUpdate` (`self.downMesh`) "/Game/Meshes/Weapon/Modular/Gungnir/Base/Gungnir_headDown.Gungnir_headDown" false)
          (set `self.AbilityToAdd` "/Game/Blueprints/Abilities/BP_Teleport.BP_Teleport_C"))
        (:`NewEnumerator2`
          (`SkinnedMeshComponent.SetSkinnedAssetAndUpdate` (`self.downMesh`) "/Game/Meshes/Weapon/Modular/Axe/Basic/axe_basicBLADE.axe_basicBLADE" false)
          (set `self.AbilityToAdd` "/Game/Blueprints/Abilities/BP_Sacriface.BP_Sacriface_C")))
      (if (`KismetArrayLibrary.Array_IsValidIndex` _knownabilities_2 1)
        (`KismetArrayLibrary.Array_Set` _knownabilities_2 1 (`self.AbilityToAdd`))
        (else
          (`KismetArrayLibrary.Array_Add` _knownabilities_2 (`self.AbilityToAdd`))))
      (`/Game/Blueprints/Abilities/BPC_Ability.InitAbilities` (`/Game/Blueprints/BP_ThirdPersonCharacter.BPC_Ability` (`self.Player`)) _knownabilities_2))))

(fn `UserConstructionScript`
  (`parent.UserConstructionScript`)
  (`SkinnedMeshComponent.SetLeaderPoseComponent` (`self.HeadMesh`) (`self.WeaponMesh`) false)
  (`SkinnedMeshComponent.SetLeaderPoseComponent` (`self.CubesHeadMesh`) (`self.WeaponMesh`) false)
  (`SkinnedMeshComponent.SetLeaderPoseComponent` (`self.downMesh`) (`self.WeaponMesh`) false))