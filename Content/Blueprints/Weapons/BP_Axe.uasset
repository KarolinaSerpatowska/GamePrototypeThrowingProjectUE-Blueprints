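; Throwable axe weapon that spins in flight, lodges where it lands and cannot be teleported to.
; Fire detaches it, adds projectile movement at a charge-scaled speed, starts tracing and spins the pivot by timeline.
; Landing removes the projectile component, sets position and randomized tilt from the impact normal, and enables pickup collision.
; ChangeWeaponParts swaps base and blade meshes; the base choice also sets a player ability slot (Stun or none).
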(event `self.ReceiveBeginPlay`
  (`parent.ReceiveBeginPlay`))

(event `StartRotation`
  (`TimelineComponent.SetPlayRate` (`self.AxeRotation`) (`self.RotationRate`))
  (bind (_direction _newtrack_0) (`Timeline|AxeRotation` :!via `PlayFromStart` :!label _label)
    (:`Update`
      (`SceneComponent.K2_SetRelativeRotation` (`self.Pivot`) (`KismetMathLibrary.MakeRotator` 0.0 (* _newtrack_0 -360.0)) false false))))

(event `StopRot`
  (goto _label :!via `Stop`))

(event `self.StopRotation`
  (`self.StopRot`)
  (`SceneComponent.K2_SetRelativeRotation` :`self` (`self.Pivot`)))

(event `/Game/Blueprints/Weapons/BPI_ThrowableWeapon.Fire`
  (params (AimDirection :type "Vector Structure") (InitialRotation :type "Rotator Structure") (CameraLocation :type "Vector Structure"))
  (`self.K2_DetachFromActor` "KeepWorld" "KeepWorld" "KeepWorld")
  (`self.K2_SetActorRotation` (`KismetMathLibrary.MakeRotator` (+ 0.0 (.roll (`self.InitialRotation`))) (.pitch (`self.InitialRotation`)) (.yaw (`self.InitialRotation`))))
  (set `self.InitialRotation` InitialRotation)
  (set `self.ThrowDirection` (`KismetMathLibrary.InverseTransformDirection` (`self.GetTransform`) AimDirection))
  (set `self.WeaponState` "NewEnumerator1")
  (`PrimitiveComponent.SetCollisionResponseToChannel` (`self.WeaponMesh`) "ECC_WorldStatic" "ECR_Block")
  (bind _returnvalue (`AddComponent|NODE_AddProjectileMovementComponent-0`))
  (bind _output_get (set `self.ProjectileMovement` _returnvalue))
  (`self.StartRotation`)
  (set `ProjectileMovementComponent.ProjectileGravityScale` 1.0 _output_get)
  (`ProjectileMovementComponent.SetVelocityInLocalSpace` _output_get (* (`self.ThrowDirection`) (`KismetMathLibrary.Lerp` (`self.MinCharge`) (`self.MaxCharge`) (`self.ThrowChargeAmount`))))
  (set `self.ThrowChargeAmount` 0.0)
  (`self.StopCharge`)
  (`self.StartTracing`))

(event `self.LandWeapon`
  (`ActorComponent.K2_DestroyComponent` (`self.ProjectileMovement`))
  (`self.LodgeWithRotation`)
  (`PrimitiveComponent.SetCollisionEnabled` (`self.PickupCollision`) "QueryAndPhysics"))

(fn `AdjustImpactPitch`
  (params (ImpactNormal :type "Vector Structure") (InclinedSurfaceRange :type "Float (double-precision)") (RegularSurfaceRange :type "Float (double-precision)"))
  (returns (ReturnValue :type "Float (double-precision)"))
  (bind (_returnvalue_roll _returnvalue_pitch) (`KismetMathLibrary.BreakRotator` (`KismetMathLibrary.MakeRotationFromAxes` ImpactNormal)))
  (return (- (`KismetMathLibrary.SelectFloat` RegularSurfaceRange InclinedSurfaceRange (> _returnvalue_pitch 0.0)) _returnvalue_pitch)))

(fn `CanTeleportTo`
  (returns (CanTeleport :type Boolean))
  (return false))

(fn `ChangeWeaponParts`
  (bind (_weaponinfo_weapontype _weaponinfo_canbethrown _weaponinfo_weaponname _weaponinfo_baseselection _weaponinfo_bladeselection) (break `/Game/Blueprints/Weapons/S_WeaponInfo` (`self.WeaponInfo`)))
  (bind _knownabilities (`/Game/Blueprints/BP_ThirdPersonCharacter.KnownAbilities` (`self.Player`)))
  (`parent.ChangeWeaponParts`)
  (`|ExecutionSequence`
    (:`then_0`
      (switch `/Game/Blueprints/Weapons/Enum_BaseSelection` _weaponinfo_baseselection
        (:`NewEnumerator0`
          (`SkinnedMeshComponent.SetSkinnedAssetAndUpdate` (`self.WeaponMesh`) "/Game/Meshes/Weapon/Modular/Axe/Basic/axe_basic.axe_basic" false)
          (set `self.AbilityToAdd` null))
        (:`NewEnumerator2`
          (`SkinnedMeshComponent.SetSkinnedAssetAndUpdate` (`self.WeaponMesh`) "/Game/Meshes/Weapon/Modular/Axe/Better/axe_better.axe_better" false)
          (set `self.AbilityToAdd` "/Game/Blueprints/Abilities/BP_Stun.BP_Stun_C")))
      (if (`KismetArrayLibrary.Array_IsValidIndex` _knownabilities 3)
        (`KismetArrayLibrary.Array_Set` _knownabilities 3 (`self.AbilityToAdd`))
        (else
          (`KismetArrayLibrary.Array_Add` _knownabilities (`self.AbilityToAdd`))))
      (`/Game/Blueprints/Abilities/BPC_Ability.InitAbilities` (`/Game/Blueprints/BP_ThirdPersonCharacter.BPC_Ability` (`self.Player`)) _knownabilities))
    (:`then_1`
      (switch `/Game/Blueprints/Weapons/Enum_BladeSelection` _weaponinfo_bladeselection
        (:`NewEnumerator0`
          (`SkinnedMeshComponent.SetSkinnedAssetAndUpdate` (`self.Blade`) "/Game/Meshes/Weapon/Modular/Axe/Basic/axe_basicBLADE.axe_basicBLADE" false))
        (:`NewEnumerator1`
          (`SkinnedMeshComponent.SetSkinnedAssetAndUpdate` (`self.Blade`) "/Game/Meshes/Weapon/Modular/Axe/Better/axe_betterBlade.axe_betterBlade" false))))))

(fn `LodgeWithRotation`
  (`KismetSystemLibrary.PrintString` "lodge")
  (`self.StopRotation`)
  (`SceneComponent.K2_SetRelativeRotation` :`self` (`self.Pivot`))
  (`self.K2_SetActorRotation` (`self.InitialRotation`))
  (`SceneComponent.K2_SetRelativeRotation` (`self.LodgePoint`) (`KismetMathLibrary.MakeRotator` (`KismetMathLibrary.RandomFloatInRange` -3.0 -8.0) (`self.AdjustImpactPitch` (`self.ImpactNormal`) (`KismetMathLibrary.RandomFloatInRange` -30.0 -55.0) (`KismetMathLibrary.RandomFloatInRange` -5.0 -25.0))) false false)
  (`self.K2_SetActorLocation` (`self.AdjustImpactLocation` (`self.ImpactNormal`) (`self.ImpactPoint`)))
  (set `self.WeaponState` "NewEnumerator2")
  (set `self.WeaponMainState` "NewEnumerator0"))

(fn `UserConstructionScript`
  (`parent.UserConstructionScript`)
  (`SkinnedMeshComponent.SetLeaderPoseComponent` (`self.Blade`) (`self.WeaponMesh`) false))