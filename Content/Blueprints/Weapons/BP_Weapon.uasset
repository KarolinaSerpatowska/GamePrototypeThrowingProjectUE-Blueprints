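; Weapon actor for modular spears and axes that the player picks up, carries and equips.
; Overlapping the pickup registers it with the player's inventory component, destroying the actor if it cannot be equipped.
; Equip and UnEquip snap it between hand and carry sockets, updating its state and the AnimBP weapon type.
; GetDamage and GetResistance sum DataTable stats per selected part; ChangeWeaponParts is empty and CanThrow returns false.
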(event `self.ReceiveBeginPlay`
  (set `self.WeaponMainState` "NewEnumerator0")
  (if (not (`.IsEquipped_18_BC53C1EA4922E0947D4915BE540F2BBA` (break `/Game/Blueprints/Weapons/S_WeaponInfo` (`self.WeaponInfo`))))
    (`PrimitiveComponent.SetCollisionEnabled` (`self.WeaponItemPickup`) "QueryAndPhysics")))

(event `Equip`
  (bind _weaponinfo_weapontype (break `/Game/Blueprints/Weapons/S_WeaponInfo` (`self.WeaponInfo`)))
  (bind _canequip (message `/Game/Blueprints/Weapons/BPI_ThrowableWeapon.CanBeEquiped` self))
  (if _canequip
    (bind _skeletalmesh (`/Game/Blueprints/BPI_CharacterUtilityFunc.GetMesh` (`self.Player`)))
    (`self.K2_AttachToComponent` _skeletalmesh (`self.EqupiSocketName`) "SnapToTarget" "SnapToTarget" "SnapToTarget")
    (set `self.IsInHand` true)
    (`self.EquipWeapon`)
    (set `/Game/Animations/ABP_Player.WeaponType` _weaponinfo_weapontype (`/Game/Blueprints/BP_ThirdPersonCharacter.AnimBP` (`self.Player`)))))

(event `UnEquip`
  (bind _skeletalmesh (`/Game/Blueprints/BPI_CharacterUtilityFunc.GetMesh` (`self.Player`)))
  (`self.K2_AttachToComponent` _skeletalmesh (`/Game/Blueprints/MyFunctionLibrary.GetSocketNameByPoint` (`self.CurrentAttachPoint`)) "SnapToTarget" "SnapToTarget" "SnapToTarget")
  (set `self.IsInHand` false)
  (`self.UnequipWeapon`)
  (set `/Game/Animations/ABP_Player.WeaponType` "NewEnumerator3" (`/Game/Blueprints/BP_ThirdPersonCharacter.AnimBP` (`self.Player`))))

(event `self.WeaponItemPickup.OnComponentBeginOverlap`
  (params (OverlappedComponent :type "PrimitiveComponent Object Reference") (OtherActor :type "Actor Object Reference") (OtherComp :type "PrimitiveComponent Object Reference") (OtherBodyIndex :type Integer) (bFromSweep :type Boolean) (SweepResult :type "HitResult Structure (by ref)"))
  (bind (_weapontype _canbethrown _weaponname _baseselection _bladeselection _isequipped _somethingselection _bladedownselection _weaponclass) (break `/Game/Blueprints/Weapons/S_WeaponInfo` (`self.WeaponInfo`)))
  (bind _returnvalue (`GameplayStatics.GetObjectClass` self))
  (bind _player (message `/Game/Blueprints/BPI_CharacterUtilityFunc.GetPlayer` OtherActor))
  (`/Engine/EditorBlueprintResources/StandardMacros.IsValid` _player
    (:`Is Valid`
      (bind _output_get (set `self.Player` _player))
      (bind _bpc_inventorymenager (`/Game/Blueprints/BP_ThirdPersonCharacter.BPC_InventoryMenager` _output_get))
      (bind _can (`/Game/Blueprints/Inventory/BPC_InventoryMenager.CanEquipPickedWeapon` _bpc_inventorymenager))
      (if _can
        (if (not (`self.PickedUP`))
          (for _array_element (`/Game/Blueprints/Inventory/BPC_InventoryMenager.OwnedWeapons` _bpc_inventorymenager)
            (if (== (`GameplayStatics.GetObjectClass` self) _array_element)
              (set `self.PickedUP` true)
              (break)))
          (if (not (`self.PickedUP`))
            (`KismetArrayLibrary.Array_Add` (`/Game/Blueprints/Inventory/BPC_InventoryMenager.OwnedWeapons` _bpc_inventorymenager) (`GameplayStatics.GetObjectClass` self)))
          (`/Game/Blueprints/Inventory/BPC_InventoryMenager.AddToInventory` _bpc_inventorymenager self (`self.WeaponInfo`))
          (`PrimitiveComponent.SetCollisionEnabled` (`self.WeaponItemPickup`) "NoCollision")
          (`/Game/Blueprints/Inventory/BPC_InventoryMenager.UpdateWeaponInfos` (`/Game/Blueprints/BP_ThirdPersonCharacter.BPC_InventoryMenager` (`self.Player`)) (make `/Game/Blueprints/Weapons/S_WeaponInfo` _weapontype _canbethrown _weaponname _baseselection _bladeselection true _somethingselection _bladedownselection _weaponclass))
          (`ActorComponent.K2_DestroyComponent` (`self.WeaponItemPickup`)))
        (else
          (`KismetArrayLibrary.Array_Add` (`/Game/Blueprints/Inventory/BPC_InventoryMenager.OwnedWeapons` _bpc_inventorymenager) _returnvalue)
          (`/Game/Blueprints/Inventory/BPC_InventoryMenager.UpdateWeaponInfos` (`/Game/Blueprints/BP_ThirdPersonCharacter.BPC_InventoryMenager` (`self.Player`)) (`.WeaponInfo` (defaults `Object` _returnvalue)))
          (set `self.PickedUP` true)
          (`self.K2_DestroyActor`))))))

(fn `Attach Weapon to Character`
  (params (SocketName :type Name))
  (bind (_weaponinfo_weapontype _weaponinfo_canbethrown _weaponinfo_weaponname _weaponinfo_baseselection _weaponinfo_bladeselection _weaponinfo_isequipped _weaponinfo_somethingselection _weaponinfo_bladedownselection _weaponinfo_weaponclass) (break `/Game/Blueprints/Weapons/S_WeaponInfo` (`self.WeaponInfo`)))
  (bind _skeletalmesh (`/Game/Blueprints/BPI_CharacterUtilityFunc.GetMesh` (`self.Player`)))
  (if (`SceneComponent.DoesSocketExist` _skeletalmesh SocketName)
    (`self.K2_AttachToComponent` _skeletalmesh SocketName "SnapToTarget" "SnapToTarget" "SnapToTarget")
    (set `self.CurrentAttachPoint` (`/Game/Blueprints/MyFunctionLibrary.GetPointNameBySocket` SocketName))
    (set `self.WeaponInfo` (make `/Game/Blueprints/Weapons/S_WeaponInfo` _weaponinfo_weapontype _weaponinfo_canbethrown _weaponinfo_weaponname _weaponinfo_baseselection _weaponinfo_bladeselection true _weaponinfo_somethingselection _weaponinfo_bladedownselection _weaponinfo_weaponclass))))

(fn `CanThrow`
  (returns (CanThrow :type Boolean))
  (return false))

(fn `ChangeWeaponParts`)

(fn `EquipWeapon`
  (set `self.WeaponMainState` "NewEnumerator1"))

(fn `GetDamage`
  (returns (BaseDmg :type "Float (double-precision)") (Thrust :type "Float (double-precision)") (Slash :type "Float (double-precision)"))
  (locals (LocalDmg :type "Float (double-precision)") (LocalThrust :type "Float (double-precision)") (LocalSlash :type "Float (double-precision)"))
  (bind (_weapontype _canbethrown _weaponname _baseselection _bladeselection _isequipped _somethingselection _bladedownselection) (break `/Game/Blueprints/Weapons/S_WeaponInfo` (`self.WeaponInfo`)))
  (switch `/Game/Blueprints/Weapons/Enum_Weapons` _weapontype
    (:`NewEnumerator1`
      (`|ExecutionSequence`
        (:`then_0`
          (switch `/Game/Blueprints/Weapons/Enum_BaseSelection` _baseselection
            (:`NewEnumerator0`
              (bind _returnvalue (`|GetDataTableRow` "/Game/Blueprints/Weapons/SpearModules.SpearModules" "Base_Basic")
                (:`then`
                  (bind (_dmg _thrust _slash) (break `/Game/Blueprints/Weapons/S_ModuleStats` (`.Stats_25_2B3F836C454AE7F53217E5BB6CFF5EBD` (break `/Game/Blueprints/Weapons/S_ModuleInfo` _returnvalue))))
                  (set `local.LocalDmg` (+ (`local.LocalDmg`) _dmg))
                  (set `local.LocalThrust` (+ (`local.LocalThrust`) _thrust))
                  (set `local.LocalSlash` (+ (`local.LocalSlash`) _slash)))))
            (:`NewEnumerator2`
              (bind _returnvalue_2 (`|GetDataTableRow` "/Game/Blueprints/Weapons/SpearModules.SpearModules" "Base_better")
                (:`then`
                  (bind (_dmg_2 _thrust_2 _slash_2) (break `/Game/Blueprints/Weapons/S_ModuleStats` (`.Stats_25_2B3F836C454AE7F53217E5BB6CFF5EBD` (break `/Game/Blueprints/Weapons/S_ModuleInfo` _returnvalue_2))))
                  (set `local.LocalDmg` (+ (`local.LocalDmg`) _dmg_2))
                  (set `local.LocalThrust` (+ (`local.LocalThrust`) _thrust_2))
                  (set `local.LocalSlash` (+ (`local.LocalSlash`) _slash_2)))))))
        (:`then_1`
          (switch `/Game/Blueprints/Weapons/Enum_BladeSelection` _bladeselection
            (:`NewEnumerator0`
              (bind _returnvalue_3 (`|GetDataTableRow` "/Game/Blueprints/Weapons/SpearModules.SpearModules" "Blade_Basic")
                (:`then`
                  (bind (_dmg_3 _thrust_3 _slash_3) (break `/Game/Blueprints/Weapons/S_ModuleStats` (`.Stats_25_2B3F836C454AE7F53217E5BB6CFF5EBD` (break `/Game/Blueprints/Weapons/S_ModuleInfo` _returnvalue_3))))
                  (set `local.LocalDmg` (+ (`local.LocalDmg`) _dmg_3))
                  (set `local.LocalThrust` (+ (`local.LocalThrust`) _thrust_3))
                  (set `local.LocalSlash` (+ (`local.LocalSlash`) _slash_3)))))
            (:`NewEnumerator1`
              (bind _returnvalue_4 (`|GetDataTableRow` "/Game/Blueprints/Weapons/SpearModules.SpearModules" "Blade_better")
                (:`then`
                  (bind (_dmg_4 _thrust_4 _slash_4) (break `/Game/Blueprints/Weapons/S_ModuleStats` (`.Stats_25_2B3F836C454AE7F53217E5BB6CFF5EBD` (break `/Game/Blueprints/Weapons/S_ModuleInfo` _returnvalue_4))))
                  (set `local.LocalDmg` (+ (`local.LocalDmg`) _dmg_4))
                  (set `local.LocalThrust` (+ (`local.LocalThrust`) _thrust_4))
                  (set `local.LocalSlash` (+ (`local.LocalSlash`) _slash_4)))))))
        (:`then_2`
          (switch `/Game/Blueprints/Weapons/Enum_SomethingSelection` _somethingselection
            (:`NewEnumerator0`
              (bind _returnvalue_5 (`|GetDataTableRow` "/Game/Blueprints/Weapons/SpearModules.SpearModules" "Something_Basic")
                (:`then`
                  (bind (_dmg_5 _thrust_5 _slash_5) (break `/Game/Blueprints/Weapons/S_ModuleStats` (`.Stats_25_2B3F836C454AE7F53217E5BB6CFF5EBD` (break `/Game/Blueprints/Weapons/S_ModuleInfo` _returnvalue_5))))
                  (set `local.LocalDmg` (+ (`local.LocalDmg`) _dmg_5))
                  (set `local.LocalThrust` (+ (`local.LocalThrust`) _thrust_5))
                  (set `local.LocalSlash` (+ (`local.LocalSlash`) _slash_5)))))
            (:`NewEnumerator2`
              (bind _returnvalue_6 (`|GetDataTableRow` "/Game/Blueprints/Weapons/SpearModules.SpearModules" "Something_better")
                (:`then`
                  (bind (_dmg_6 _thrust_6 _slash_6) (break `/Game/Blueprints/Weapons/S_ModuleStats` (`.Stats_25_2B3F836C454AE7F53217E5BB6CFF5EBD` (break `/Game/Blueprints/Weapons/S_ModuleInfo` _returnvalue_6))))
                  (set `local.LocalDmg` (+ (`local.LocalDmg`) _dmg_6))
                  (set `local.LocalThrust` (+ (`local.LocalThrust`) _thrust_6))
                  (set `local.LocalSlash` (+ (`local.LocalSlash`) _slash_6)))))))
        (:`then_3`
          (switch `/Game/Blueprints/Weapons/Enum_BladeDownSelection` _bladedownselection
            (:`NewEnumerator0`
              (bind _returnvalue_7 (`|GetDataTableRow` "/Game/Blueprints/Weapons/SpearModules.SpearModules" "BladeDown_Basic")
                (:`then`
                  (bind (_dmg_7 _thrust_7 _slash_7) (break `/Game/Blueprints/Weapons/S_ModuleStats` (`.Stats_25_2B3F836C454AE7F53217E5BB6CFF5EBD` (break `/Game/Blueprints/Weapons/S_ModuleInfo` _returnvalue_7))))
                  (set `local.LocalDmg` (+ (`local.LocalDmg`) _dmg_7))
                  (set `local.LocalThrust` (+ (`local.LocalThrust`) _thrust_7))
                  (set `local.LocalSlash` (+ (`local.LocalSlash`) _slash_7)))))
            (:`NewEnumerator2`
              (bind _returnvalue_8 (`|GetDataTableRow` "/Game/Blueprints/Weapons/SpearModules.SpearModules" "BladeDown_better")
                (:`then`
                  (bind (_dmg_8 _thrust_8 _slash_8) (break `/Game/Blueprints/Weapons/S_ModuleStats` (`.Stats_25_2B3F836C454AE7F53217E5BB6CFF5EBD` (break `/Game/Blueprints/Weapons/S_ModuleInfo` _returnvalue_8))))
                  (set `local.LocalDmg` (+ (`local.LocalDmg`) _dmg_8))
                  (set `local.LocalThrust` (+ (`local.LocalThrust`) _thrust_8))
                  (set `local.LocalSlash` (+ (`local.LocalSlash`) _slash_8)))))))
        (:`then_4`
          (return (`local.LocalDmg`) (`local.LocalThrust`) (`local.LocalSlash`)))))
    (:`NewEnumerator2`
      (`|ExecutionSequence`
        (:`then_0`
          (switch `/Game/Blueprints/Weapons/Enum_BaseSelection` _baseselection
            (:`NewEnumerator0`
              (bind _returnvalue_9 (`|GetDataTableRow` "/Game/Blueprints/Weapons/AxeModules.AxeModules" "Base_Basic")
                (:`then`
                  (bind (_dmg_9 _thrust_9 _slash_9) (break `/Game/Blueprints/Weapons/S_ModuleStats` (`.Stats_25_2B3F836C454AE7F53217E5BB6CFF5EBD` (break `/Game/Blueprints/Weapons/S_ModuleInfo` _returnvalue_9))))
                  (set `local.LocalDmg` (+ (`local.LocalDmg`) _dmg_9))
                  (set `local.LocalThrust` (+ (`local.LocalThrust`) _thrust_9))
                  (set `local.LocalSlash` (+ (`local.LocalSlash`) _slash_9)))))
            (:`NewEnumerator2`
              (bind _returnvalue_10 (`|GetDataTableRow` "/Game/Blueprints/Weapons/AxeModules.AxeModules" "Base_Better")
                (:`then`
                  (bind (_dmg_10 _thrust_10 _slash_10) (break `/Game/Blueprints/Weapons/S_ModuleStats` (`.Stats_25_2B3F836C454AE7F53217E5BB6CFF5EBD` (break `/Game/Blueprints/Weapons/S_ModuleInfo` _returnvalue_10))))
                  (set `local.LocalDmg` (+ (`local.LocalDmg`) _dmg_10))
                  (set `local.LocalThrust` (+ (`local.LocalThrust`) _thrust_10))
                  (set `local.LocalSlash` (+ (`local.LocalSlash`) _slash_10)))))))
        (:`then_1`
          (switch `/Game/Blueprints/Weapons/Enum_BladeSelection` _bladeselection
            (:`NewEnumerator0`
              (bind _returnvalue_11 (`|GetDataTableRow` "/Game/Blueprints/Weapons/AxeModules.AxeModules" "Blade_Basic")
                (:`then`
                  (bind (_dmg_11 _thrust_11 _slash_11) (break `/Game/Blueprints/Weapons/S_ModuleStats` (`.Stats_25_2B3F836C454AE7F53217E5BB6CFF5EBD` (break `/Game/Blueprints/Weapons/S_ModuleInfo` _returnvalue_11))))
                  (set `local.LocalDmg` (+ (`local.LocalDmg`) _dmg_11))
                  (set `local.LocalThrust` (+ (`local.LocalThrust`) _thrust_11))
                  (set `local.LocalSlash` (+ (`local.LocalSlash`) _slash_11)))))
            (:`NewEnumerator1`
              (bind _returnvalue_12 (`|GetDataTableRow` "/Game/Blueprints/Weapons/AxeModules.AxeModules" "Blade_Better")
                (:`then`
                  (bind (_dmg_12 _thrust_12 _slash_12) (break `/Game/Blueprints/Weapons/S_ModuleStats` (`.Stats_25_2B3F836C454AE7F53217E5BB6CFF5EBD` (break `/Game/Blueprints/Weapons/S_ModuleInfo` _returnvalue_12))))
                  (set `local.LocalDmg` (+ (`local.LocalDmg`) _dmg_12))
                  (set `local.LocalThrust` (+ (`local.LocalThrust`) _thrust_12))
                  (set `local.LocalSlash` (+ (`local.LocalSlash`) _slash_12)))))))
        (:`then_2`
          (return (`local.LocalDmg`) (`local.LocalThrust`) (`local.LocalSlash`)))))))

(fn `GetDmgLocations`
  (returns (DmgLocations :type "Array of /Game/Blueprints/Weapons/S_DmgLocations Structure"))
  (return (`|MakeArray` (make `/Game/Blueprints/Weapons/S_DmgLocations` (`SceneComponent.K2_GetComponentLocation` (`self.DmgA`)) (`SceneComponent.K2_GetComponentLocation` (`self.DmgB`))))))

(fn `GetResistance`
  (returns (ResistanceThrust :type "Float (double-precision)") (ResistanceSlash :type "Float (double-precision)"))
  (locals (localThrust :type "Float (double-precision)") (localSlash :type "Float (double-precision)"))
  (bind (_weapontype _canbethrown _weaponname _baseselection _bladeselection _isequipped _somethingselection _bladedownselection) (break `/Game/Blueprints/Weapons/S_WeaponInfo` (`self.WeaponInfo`)))
  (switch `/Game/Blueprints/Weapons/Enum_Weapons` _weapontype
    (:`NewEnumerator1`
      (`|ExecutionSequence`
        (:`then_0`
          (switch `/Game/Blueprints/Weapons/Enum_BaseSelection` _baseselection
            (:`NewEnumerator0`
              (bind _returnvalue (`|GetDataTableRow` "/Game/Blueprints/Weapons/SpearModules.SpearModules" "Base_Basic")
                (:`then`
                  (bind (_dmg _thrust _slash _blockorarmorthrust _blockorarmorslash) (break `/Game/Blueprints/Weapons/S_ModuleStats` (`.Stats_25_2B3F836C454AE7F53217E5BB6CFF5EBD` (break `/Game/Blueprints/Weapons/S_ModuleInfo` _returnvalue))))
                  (set `local.localThrust` (+ (`local.localThrust`) _blockorarmorthrust))
                  (set `local.localSlash` (+ (`local.localSlash`) _blockorarmorslash)))))
            (:`NewEnumerator2`
              (bind _returnvalue_2 (`|GetDataTableRow` "/Game/Blueprints/Weapons/SpearModules.SpearModules" "Base_better")
                (:`then`
                  (bind (_dmg_2 _thrust_2 _slash_2 _blockorarmorthrust_2 _blockorarmorslash_2) (break `/Game/Blueprints/Weapons/S_ModuleStats` (`.Stats_25_2B3F836C454AE7F53217E5BB6CFF5EBD` (break `/Game/Blueprints/Weapons/S_ModuleInfo` _returnvalue_2))))
                  (set `local.localThrust` (+ (`local.localThrust`) _blockorarmorthrust_2))
                  (set `local.localSlash` (+ (`local.localSlash`) _blockorarmorslash_2)))))))
        (:`then_1`
          (switch `/Game/Blueprints/Weapons/Enum_BladeSelection` _bladeselection
            (:`NewEnumerator0`
              (bind _returnvalue_3 (`|GetDataTableRow` "/Game/Blueprints/Weapons/SpearModules.SpearModules" "Blade_Basic")
                (:`then`
                  (bind (_dmg_3 _thrust_3 _slash_3 _blockorarmorthrust_3 _blockorarmorslash_3) (break `/Game/Blueprints/Weapons/S_ModuleStats` (`.Stats_25_2B3F836C454AE7F53217E5BB6CFF5EBD` (break `/Game/Blueprints/Weapons/S_ModuleInfo` _returnvalue_3))))
                  (set `local.localThrust` (+ (`local.localThrust`) _blockorarmorthrust_3))
                  (set `local.localSlash` (+ (`local.localSlash`) _blockorarmorslash_3)))))
            (:`NewEnumerator1`
              (bind _returnvalue_4 (`|GetDataTableRow` "/Game/Blueprints/Weapons/SpearModules.SpearModules" "Blade_better")
                (:`then`
                  (bind (_dmg_4 _thrust_4 _slash_4 _blockorarmorthrust_4 _blockorarmorslash_4) (break `/Game/Blueprints/Weapons/S_ModuleStats` (`.Stats_25_2B3F836C454AE7F53217E5BB6CFF5EBD` (break `/Game/Blueprints/Weapons/S_ModuleInfo` _returnvalue_4))))
                  (set `local.localThrust` (+ (`local.localThrust`) _blockorarmorthrust_4))
                  (set `local.localSlash` (+ (`local.localSlash`) _blockorarmorslash_4)))))))
        (:`then_2`
          (switch `/Game/Blueprints/Weapons/Enum_SomethingSelection` _somethingselection
            (:`NewEnumerator0`
              (bind _returnvalue_5 (`|GetDataTableRow` "/Game/Blueprints/Weapons/SpearModules.SpearModules" "Something_Basic")
                (:`then`
                  (bind (_dmg_5 _thrust_5 _slash_5 _blockorarmorthrust_5 _blockorarmorslash_5) (break `/Game/Blueprints/Weapons/S_ModuleStats` (`.Stats_25_2B3F836C454AE7F53217E5BB6CFF5EBD` (break `/Game/Blueprints/Weapons/S_ModuleInfo` _returnvalue_5))))
                  (set `local.localThrust` (+ (`local.localThrust`) _blockorarmorthrust_5))
                  (set `local.localSlash` (+ (`local.localSlash`) _blockorarmorslash_5)))))
            (:`NewEnumerator2`
              (bind _returnvalue_6 (`|GetDataTableRow` "/Game/Blueprints/Weapons/SpearModules.SpearModules" "Something_better")
                (:`then`
                  (bind (_dmg_6 _thrust_6 _slash_6 _blockorarmorthrust_6 _blockorarmorslash_6) (break `/Game/Blueprints/Weapons/S_ModuleStats` (`.Stats_25_2B3F836C454AE7F53217E5BB6CFF5EBD` (break `/Game/Blueprints/Weapons/S_ModuleInfo` _returnvalue_6))))
                  (set `local.localThrust` (+ (`local.localThrust`) _blockorarmorthrust_6))
                  (set `local.localSlash` (+ (`local.localSlash`) _blockorarmorslash_6)))))))
        (:`then_3`
          (switch `/Game/Blueprints/Weapons/Enum_BladeDownSelection` _bladedownselection
            (:`NewEnumerator0`
              (bind _returnvalue_7 (`|GetDataTableRow` "/Game/Blueprints/Weapons/SpearModules.SpearModules" "BladeDown_Basic")
                (:`then`
                  (bind (_dmg_7 _thrust_7 _slash_7 _blockorarmorthrust_7 _blockorarmorslash_7) (break `/Game/Blueprints/Weapons/S_ModuleStats` (`.Stats_25_2B3F836C454AE7F53217E5BB6CFF5EBD` (break `/Game/Blueprints/Weapons/S_ModuleInfo` _returnvalue_7))))
                  (set `local.localThrust` (+ (`local.localThrust`) _blockorarmorthrust_7))
                  (set `local.localSlash` (+ (`local.localSlash`) _blockorarmorslash_7)))))
            (:`NewEnumerator2`
              (bind _returnvalue_8 (`|GetDataTableRow` "/Game/Blueprints/Weapons/SpearModules.SpearModules" "BladeDown_better")
                (:`then`
                  (bind (_dmg_8 _thrust_8 _slash_8 _blockorarmorthrust_8 _blockorarmorslash_8) (break `/Game/Blueprints/Weapons/S_ModuleStats` (`.Stats_25_2B3F836C454AE7F53217E5BB6CFF5EBD` (break `/Game/Blueprints/Weapons/S_ModuleInfo` _returnvalue_8))))
                  (set `local.localThrust` (+ (`local.localThrust`) _blockorarmorthrust_8))
                  (set `local.localSlash` (+ (`local.localSlash`) _blockorarmorslash_8)))))))
        (:`then_4`
          (return (`local.localThrust`) (`local.localSlash`)))))
    (:`NewEnumerator2`
      (`|ExecutionSequence`
        (:`then_0`
          (switch `/Game/Blueprints/Weapons/Enum_BaseSelection` _baseselection
            (:`NewEnumerator0`
              (bind _returnvalue_9 (`|GetDataTableRow` "/Game/Blueprints/Weapons/AxeModules.AxeModules" "Base_Basic")
                (:`then`
                  (bind (_dmg_9 _thrust_9 _slash_9 _blockorarmorthrust_9 _blockorarmorslash_9) (break `/Game/Blueprints/Weapons/S_ModuleStats` (`.Stats_25_2B3F836C454AE7F53217E5BB6CFF5EBD` (break `/Game/Blueprints/Weapons/S_ModuleInfo` _returnvalue_9))))
                  (set `local.localThrust` (+ (`local.localThrust`) _blockorarmorthrust_9))
                  (set `local.localSlash` (+ (`local.localSlash`) _blockorarmorslash_9)))))
            (:`NewEnumerator2`
              (bind _returnvalue_10 (`|GetDataTableRow` "/Game/Blueprints/Weapons/AxeModules.AxeModules" "Base_Better")
                (:`then`
                  (bind (_dmg_10 _thrust_10 _slash_10 _blockorarmorthrust_10 _blockorarmorslash_10) (break `/Game/Blueprints/Weapons/S_ModuleStats` (`.Stats_25_2B3F836C454AE7F53217E5BB6CFF5EBD` (break `/Game/Blueprints/Weapons/S_ModuleInfo` _returnvalue_10))))
                  (set `local.localThrust` (+ (`local.localThrust`) _blockorarmorthrust_10))
                  (set `local.localSlash` (+ (`local.localSlash`) _blockorarmorslash_10)))))))
        (:`then_1`
          (switch `/Game/Blueprints/Weapons/Enum_BladeSelection` _bladeselection
            (:`NewEnumerator0`
              (bind _returnvalue_11 (`|GetDataTableRow` "/Game/Blueprints/Weapons/AxeModules.AxeModules" "Blade_Basic")
                (:`then`
                  (bind (_dmg_11 _thrust_11 _slash_11 _blockorarmorthrust_11 _blockorarmorslash_11) (break `/Game/Blueprints/Weapons/S_ModuleStats` (`.Stats_25_2B3F836C454AE7F53217E5BB6CFF5EBD` (break `/Game/Blueprints/Weapons/S_ModuleInfo` _returnvalue_11))))
                  (set `local.localThrust` (+ (`local.localThrust`) _blockorarmorthrust_11))
                  (set `local.localSlash` (+ (`local.localSlash`) _blockorarmorslash_11)))))
            (:`NewEnumerator1`
              (bind _returnvalue_12 (`|GetDataTableRow` "/Game/Blueprints/Weapons/AxeModules.AxeModules" "Blade_Better")
                (:`then`
                  (bind (_dmg_12 _thrust_12 _slash_12 _blockorarmorthrust_12 _blockorarmorslash_12) (break `/Game/Blueprints/Weapons/S_ModuleStats` (`.Stats_25_2B3F836C454AE7F53217E5BB6CFF5EBD` (break `/Game/Blueprints/Weapons/S_ModuleInfo` _returnvalue_12))))
                  (set `local.localThrust` (+ (`local.localThrust`) _blockorarmorthrust_12))
                  (set `local.localSlash` (+ (`local.localSlash`) _blockorarmorslash_12)))))))
        (:`then_2`
          (return (`local.localThrust`) (`local.localSlash`)))))))

(fn `UnequipWeapon`
  (set `self.WeaponMainState` "NewEnumerator0"))

(fn `UserConstructionScript`)