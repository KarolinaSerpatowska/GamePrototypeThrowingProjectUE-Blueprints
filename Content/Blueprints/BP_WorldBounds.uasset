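; BP_WorldBounds is a world boundary actor that tells players when they leave or re-enter the playable area.
; Overlapping the OutBounds volume sets the player's SpawnLocation to InBounds' X and Y at the player's current Z, then calls OutOfBounds.
; Overlapping InBounds calls ReturnToArea.
; Both resolve the player through GetPlayerMessage on the overlapping actor and ignore invalid results.
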(event `self.InBounds.OnComponentBeginOverlap`
  (params (OverlappedComponent :type "PrimitiveComponent Object Reference") (OtherActor :type "Actor Object Reference") (OtherComp :type "PrimitiveComponent Object Reference") (OtherBodyIndex :type Integer) (bFromSweep :type Boolean) (SweepResult :type "HitResult Structure (by ref)"))
  (bind _player (message `/Game/Blueprints/BPI_CharacterUtilityFunc.GetPlayer` OtherActor))
  (`/Engine/EditorBlueprintResources/StandardMacros.IsValid` _player
    (:`Is Valid`
      (`/Game/Blueprints/BP_ThirdPersonCharacter.ReturnToArea` _player))))

(event `self.OutBounds.OnComponentBeginOverlap`
  (params (OverlappedComponent :type "PrimitiveComponent Object Reference") (OtherActor :type "Actor Object Reference") (OtherComp :type "PrimitiveComponent Object Reference") (OtherBodyIndex :type Integer) (bFromSweep :type Boolean) (SweepResult :type "HitResult Structure (by ref)"))
  (bind (_returnvalue_x _returnvalue_y) (`KismetMathLibrary.BreakVector` (`SceneComponent.K2_GetComponentLocation` (`self.InBounds`))))
  (bind _player (message `/Game/Blueprints/BPI_CharacterUtilityFunc.GetPlayer` OtherActor))
  (`/Engine/EditorBlueprintResources/StandardMacros.IsValid` _player
    (:`Is Valid`
      (bind (_returnvalue_x_2 _returnvalue_y_2 _returnvalue_z) (`KismetMathLibrary.BreakVector` (`self.K2_GetActorLocation` _player)))
      (set `/Game/Blueprints/BP_ThirdPersonCharacter.SpawnLocation` (`KismetMathLibrary.MakeVector` _returnvalue_x _returnvalue_y _returnvalue_z) _player)
      (`/Game/Blueprints/BP_ThirdPersonCharacter.OutOfBounds` _player))))

(fn `UserConstructionScript`)