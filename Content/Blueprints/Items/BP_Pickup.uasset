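; BP_Pickup is a world item that the third-person character collects into their inventory by pressing E while nearby.
; Its sphere overlap enables input, shows an interaction indicator widget and opens a gate for the E key, reversing all three on exit.
; On press it sends a pickup message to the overlapping actor and adds the item to its inventory manager, keeping any leftover amount or destroying itself when fully taken.
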(event `self.ReceiveBeginPlay`
  (bind _asui_interaction_indicator (cast `/Game/Widgets/UI_InteractionIndicator` (`WidgetComponent.GetUserWidgetObject` (`self.InteractionIndicator`))))
  (set `self.UI Interaction Indicator` _asui_interaction_indicator)
  (`Widget.SetVisibility` (`self.UI Interaction Indicator`) "Hidden"))

(event `Key|E`
  (params (Key :type "Key Structure"))
  (:`Pressed`
    (bind _inveneotryref (message `/Game/Blueprints/BPI_CharacterUtilityFunc.GetInventoryMeneger` (`self.OverlapedActor`)))
    (`/Engine/EditorBlueprintResources/StandardMacros.IsValid` _inveneotryref
      (:`Is Valid`
        (`/Engine/EditorBlueprintResources/StandardMacros.Gate` true :!label _label
          (:`Exit`
            (message `/Game/Blueprints/BPI_CharacterUtilityFunc.Pickup` (`self.OverlapedActor`))
            (bind (_issuccess _rest) (`/Game/Blueprints/Inventory/BPC_InventoryMenager.AddItem` _inveneotryref (`self.ItemToAdd`) (`self.Amount`)))
            (if _issuccess
              (if (> _rest 0)
                (set `self.Amount` _rest)
                (else
                  (`self.K2_DestroyActor`))))))))))

(event `self.Sphere.OnComponentBeginOverlap`
  (params (OverlappedComponent :type "PrimitiveComponent Object Reference") (OtherActor :type "Actor Object Reference") (OtherComp :type "PrimitiveComponent Object Reference") (OtherBodyIndex :type Integer) (bFromSweep :type Boolean) (SweepResult :type "HitResult Structure (by ref)"))
  (if (== (`GameplayStatics.GetObjectClass` OtherActor) "/Game/Blueprints/BP_ThirdPersonCharacter.BP_ThirdPersonCharacter_C")
    (set `self.OverlapedActor` OtherActor)
    (`self.EnableInput` (`GameplayStatics.GetPlayerController` 0))
    (`Widget.SetVisibility` (`self.UI Interaction Indicator`) "Visible")
    (goto _label :!via `Open`)))

(event `self.Sphere.OnComponentEndOverlap`
  (params (OverlappedComponent :type "PrimitiveComponent Object Reference") (OtherActor :type "Actor Object Reference") (OtherComp :type "PrimitiveComponent Object Reference") (OtherBodyIndex :type Integer))
  (if (== (`GameplayStatics.GetObjectClass` OtherActor) "/Game/Blueprints/BP_ThirdPersonCharacter.BP_ThirdPersonCharacter_C")
    (set `self.OverlapedActor` null)
    (`self.DisableInput` (`GameplayStatics.GetPlayerController` 0))
    (`Widget.SetVisibility` (`self.UI Interaction Indicator`) "Hidden")
    (goto _label :!via `Close`)))

(fn `UserConstructionScript`)