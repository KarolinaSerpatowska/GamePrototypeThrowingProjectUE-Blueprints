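; Combat component that handles melee weapon hit detection, damage and death for its owning pawn.
; The State.Attacking.Weapon tag toggles ticking, which line-traces along the equipped weapon's damage points.
; Each actor is processed once per swing; those of other classes take thrust plus slash damage adjusted by resistance.
; Incoming damage lowers Health; at zero, State.Dead triggers unpossession, a death montage and frozen animation.
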(event Custom|StartDamageDetection
  (Components|Tick|SetComponentTickEnabled true)
  (Utilities|Array|Clear (Variables|Default|GetAlreadyDamagedActors)))

(event Custom|StopDamageDetection
  (Components|Tick|SetComponentTickEnabled false))

(event Custom|DamageTaken
  (params (DamagedActor :type Actor%20Object%20Reference) (Damage :type Float%20%28single-precision%29) (DamageType :type Damage%20Type%20Object%20Reference) (InstigatedBy :type Controller%20Object%20Reference) (DamageCauser :type Actor%20Object%20Reference))
  (bind _returnvalue (Actor|GetComponentbyClass DamagedActor "/Game/Blueprints/Attributes/BPC_Attributes.BPC_Attributes_C"))
  (bind _pawnref (Variables|Default|GetPawnRef))
  (Development|PrintString "DMGGGGGGGGGG")
  (Utilities|IsValid _returnvalue
    (:Is%20Valid
      (Default|ChangeAttribute _returnvalue "(TagName=\"Attribute.Health\")" (* Damage -1.0) "NewEnumerator1" (Utilities|Struct|MakeS_WhoDoneThis _pawnref (Pawn|GetController _pawnref))))))

(event Custom|AttackWeaponChange
  (params (GameplayTagContext :type S%20Gameplay%20Context%20Structure))
  (if (GameplayTags|HasTag (.ActiveTags (Utilities|Struct|BreakS_GameplayContext GameplayTagContext)) "(TagName=\"State.Attacking.Weapon\")" true)
    (CallFunction|StartDamageDetection)
    (Development|PrintString "do dmg")
    (else
      (CallFunction|StopDamageDetection)
      (Development|PrintString "stop dmg"))))

(event Custom|AttemptDmg
  (params (DmgActor :type Actor%20Object%20Reference))
  (bind _alreadydamagedactors (Variables|Default|GetAlreadyDamagedActors))
  (if (not (Utilities|Array|ContainsItem _alreadydamagedactors 0))
    (Utilities|Array|Add _alreadydamagedactors 0)
    (bind (_basedmg _thrust _slash) (Class|BPICharacterUtilityFunc|GetDmgfromWeapon(Message) (Variables|Default|GetPawnRef)))
    (bind (_resistancethrust _resistanceslash) (Class|BPICharacterUtilityFunc|GetResistance(Message) DmgActor))
    (if (!= (Utilities|GetClass DmgActor) (Utilities|GetClass (Components|GetOwner)))
      (Development|PrintString (Utilities|String|Append "DMG: " (Utilities|String|ToString(Float) (+ (|(base*(1-((block+resistance)-critical))) _basedmg 0.0 _resistancethrust _thrust) (|(base*(1-((block+resistance)-critical))) _basedmg 0.0 _resistanceslash _slash)))))
      (Game|Damage|ApplyDamage DmgActor (+ (|(base*(1-((block+resistance)-critical))) _basedmg 0.0 _resistancethrust _thrust) (|(base*(1-((block+resistance)-critical))) _basedmg 0.0 _resistanceslash _slash)) 0 0))))

(event Custom|DeathOccured
  (params (GameplayTagContext :type S%20Gameplay%20Context%20Structure))
  (bind _returnvalue (Components|GetOwner))
  (bind _pawnref (Variables|Default|GetPawnRef))
  (bind _returnvalue_2 (Pawn|GetController _pawnref))
  (Utilities|IsValid _returnvalue_2
    (:Is%20Valid
      (Pawn|UnPossess _returnvalue_2)
      (Class|BPICharacterUtilityFunc|DisableAIMovement(Message) _returnvalue)
      (bind _skeletalmesh (Class|BPICharacterUtilityFunc|GetMesh(Message) _returnvalue))
      (Animation|Montage|MontageStop (Components|SkeletalMesh|GetAnimInstance _skeletalmesh) 0.0 0)
      (Class|BPIAnimUtility|PlayFullBody(Message) (Components|SkeletalMesh|GetAnimInstance _skeletalmesh))
      (Animation|Montage|PlayMontage _skeletalmesh (Variables|Default|GetDeathAnim)
        (:OnBlendOut
          (Variables|/Script/Engine.SkeletalMeshComponent|SetbPauseAnims _skeletalmesh true))))))

(event Custom|HealthChanged
  (params (AttributeContext :type S%20Attributes%20Context%20Structure))
  (bind (_attributechanged _valuechange _whodonethis) (Utilities|Struct|BreakS_AttributesContext AttributeContext))
  (if (<= (Utilities|Struct|BreakS_Attributes _attributechanged) 0.0)
    (Default|AddTag (Actor|GetComponentbyClass (Components|GetOwner) "/Game/Blueprints/GameplayTags/BPC_GameplayTags.BPC_GameplayTags_C") "(TagName=\"State.Dead\")" _whodonethis)))

(event EventBeginPlay
  (bind _returnvalue (Components|GetOwner))
  (bind _returnvalue_2 (Actor|GetComponentbyClass _returnvalue "/Game/Blueprints/GameplayTags/BPC_GameplayTags.BPC_GameplayTags_C"))
  (Utilities|IsValid _returnvalue_2
    (:Is%20Valid
      (Default|AddTagListener _returnvalue_2 "(TagName=\"State.Attacking.Weapon\")" (delegate Custom|AttackWeaponChange))
      (EventDispatchers|BindEventtoOnTakeAnyDamage _returnvalue (delegate Custom|DamageTaken))
      (bind _aspawn (Utilities|Casting|CastToPawn _returnvalue))
      (Variables|Default|SetPawnRef _aspawn)
      (Default|AddTagListener _returnvalue_2 "(TagName=\"State.Dead\")" (delegate Custom|DeathOccured))
      (Default|AddAtributeListener (Actor|GetComponentbyClass (Components|GetOwner) "/Game/Blueprints/Attributes/BPC_Attributes.BPC_Attributes_C") "(TagName=\"Attribute.Health\")" (delegate Custom|HealthChanged)))))

(event EventTick
  (params (DeltaSeconds :type Float%20%28single-precision%29))
  (bind _equippedweapon (Variables|Default|GetEquippedWeapon)
    (:then
      (bind _dmglocations (Class|BPIWeapon|GetDmgLocations(Message) _equippedweapon))
      (for _array_element _dmglocations
        (bind _outhits (Collision|MultiLineTraceByChannel (.Top (Utilities|Struct|BreakS_DmgLocations _array_element)) (.B (Utilities|Struct|BreakS_DmgLocations _array_element)) "TraceTypeQuery3" false 0 "Persistent" true "(R=1.000000,G=0.000000,B=0.000000,A=1.000000)" "(R=0.000000,G=1.000000,B=0.000000,A=1.000000)" 12.0))
        (for _array_element_2 _outhits
          (CallFunction|AttemptDmg (.HitActor (Collision|BreakHitResult _array_element_2))))))
    (:else)))

(fn SetEquippedWeapon
  (params (Weapon :type BP%20Weapon%20Object%20Reference))
  (Variables|Default|SetEquippedWeapon Weapon))